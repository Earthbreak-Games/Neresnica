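; Player controller for the arena game that registers a joining player and switches their view to the lobby camera.
; On possess, it caches the PlayerState name as the Steam player ID and notifies ArenaGameState that a player joined.
; It then sets the view target to the LobbyCamera of player pawn 0, cast to ThirdPersonCharacter.
; A getter exposes the stored ID as text.
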(event `self.ReceiveTick`
  (params (DeltaSeconds :type "Float (single-precision)")))

(event `self.ReceivePossess`
  (params (PossessedPawn :type "Pawn Object Reference"))
  (set `self.SteamPlayerID` (`PlayerState.GetPlayerName` (`self.PlayerState`)))
  (bind _asarena_game_state (cast `/Game/Modes_States_Instances/ArenaGameState` (`GameplayStatics.GetGameState`)))
  (`/Game/Modes_States_Instances/ArenaGameState.PlayerJoined` _asarena_game_state)
  (bind _asthird_person_character (cast `/Game/Character/Blueprints/ThirdPersonCharacter` (`GameplayStatics.GetPlayerPawn` 0)))
  (`self.SetViewTargetWithBlend` (`/Game/Character/Blueprints/ThirdPersonCharacter.LobbyCamera` _asthird_person_character)))

(fn `GetPlayerSteamID`
  (returns (SteamID :type Text))
  (return (`KismetTextLibrary.Conv_StringToText` (`self.SteamPlayerID`))))

(fn `UserConstructionScript`)