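; Gladiator is an AI-driven character Blueprint that chases a target and has placeholder melee and ranged attack events.
; Each tick, Movement moves it toward the target with SimpleMoveToActor, stopping while attacking or within melee range.
; Both attacks print a debug string, hold the attacking flag through a delay, then flag a cooldown; only melee stops movement directly.
; Missile spawning at the launch point exists but is disconnected.
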(event `self.ReceiveTick`
  (params (DeltaSeconds :type "Float (single-precision)"))
  (`self.Movement`))

(event `self.MeleeAttack`
  ;[1 1 1] No touchie!
  (set `self.mIsAttacking` true)
  (`KismetSystemLibrary.PrintString` "Melee")
  (`NavMovementComponent.StopActiveMovement` (`self.CharacterMovement`))
  ;[1 1 1] No touchie!
  (`KismetSystemLibrary.Delay` 2.0)
  (set `self.mIsAttacking` false)
  (set `self.mIsOnCooldown` true))

(event `self.RangedAttack`
  ;[1 1 1] No touchie!
  (set `self.mIsAttacking` true)
  (`KismetSystemLibrary.PrintString` "ranged")
  ;[1 1 1] No touchie!
  (`KismetSystemLibrary.Delay` 2.0)
  (set `self.mIsAttacking` false)
  (set `self.mIsOnCooldown` true))

(fn `Movement`
  (if (`self.mIsAttacking`)
    (`NavMovementComponent.StopActiveMovement` (`self.CharacterMovement`) :!label _label)
    (elif (<= (`self.mDistanceToTarget`) (`self.mMeleeRange`))
      (goto _label)
      (else
        (`AIBlueprintHelperLibrary.SimpleMoveToActor` (`self.GetController` self) (`self.mpTarget`)))))
  (return))

(fn `UserConstructionScript`)