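; Gladiator boss enemy for the arena, with melee and ranged attack flags and homing rockets aimed at the closest player character.
; On spawn it scales health by player count and round, and gets a weapon from a temporary LootSource.
; Damage and loot pass through Host-to-Client event pairs; destruction drops boss loot and updates the game state's enemy list.
; A random non-spectator targeting branch is left unconnected.
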(event `AttackConcluded`
  (set `self.IsMeleeAttacking` false)
  (set `self.IsRangedAttacking` false))

(event `RangedAttack`
  (set `self.IsRangedAttacking` true))

(event `MeleeAttack`
  (set `self.IsMeleeAttacking` true))

(event `self.ReceiveBeginPlay`
  (bind (_returnvalue_location _returnvalue_rotation) (`KismetMathLibrary.BreakTransform` (`self.GetTransform`)))
  (bind _returnvalue (`GameplayStatics.GetGameState`))
  (set `self.TargetFound` false)
  (bind _asarena_game_state (cast `/Game/Blueprints/Modes_States_Instances/ArenaGameState` _returnvalue))
  (set `self.mHealth` (`KismetMathLibrary.Conv_IntToDouble` (* (+ (* (`KismetArrayLibrary.Array_Length` (`GameStateBase.PlayerArray` _returnvalue)) 50) 100) (`/Game/Blueprints/Modes_States_Instances/ArenaGameState.RoundNum` _asarena_game_state))))
  (bind _returnvalue_2 (`|SpawnActorFromClass` "/Game/Blueprints/Loot/LootSource.LootSource_C" (`KismetMathLibrary.MakeTransform` _returnvalue_location _returnvalue_rotation) "Undefined" "OverrideRootScale" null null))
  (`/Game/Blueprints/Loot/LootSource.GenerateWeapon` _returnvalue_2 "COMMON" self)
  (`self.K2_DestroyActor` _returnvalue_2))

(event `FireMissile`
  (bind _returnvalue (`|SpawnActorFromClass` "/Game/Characters/Gladiator/Blueprints/RocketProjectile.RocketProjectile_C" (`SceneComponent.K2_GetComponentToWorld` (`self.Arrow1`)) "Undefined" "OverrideRootScale" null null))
  (bind _closest (`self.GetClosestPlayer`))
  (bind _asthird_person_character (cast `/Game/Characters/Player/Blueprints/ThirdPersonCharacter` _closest))
  (`/Game/Characters/Gladiator/Blueprints/RocketProjectile.HomingMissle` _returnvalue _asthird_person_character))

(event `HostDropLoot`
  (`self.ClientDropLoot`))

(event `HostNotifyDealDamage`
  (params (OposingUnit :type "BaseUnit Object Reference") (Damage :type "Float (double-precision)"))
  (`self.ClientDealDamage` OposingUnit Damage))

(event `ClientDealDamage`
  (params (OposingUnit :type "BaseUnit Object Reference") (Damage :type "Float (double-precision)"))
  (`self.DealDamage` OposingUnit Damage))

(event `ClientDropLoot`
  (bind (_returnvalue_location _returnvalue_rotation) (`KismetMathLibrary.BreakTransform` (`self.GetTransform`)))
  ;[1 1 1] Drop Loot
  (bind _returnvalue (`|SpawnActorFromClass` "/Game/Blueprints/Loot/LootSource.LootSource_C" (`KismetMathLibrary.MakeTransform` _returnvalue_location _returnvalue_rotation) "Undefined" "OverrideRootScale" null null))
  (set `/Game/Blueprints/Loot/LootSource.EnemyType` "BOSS" _returnvalue)
  (set `/Game/Blueprints/Loot/LootSource.BossWeapon` "Sword" _returnvalue)
  (`/Game/Blueprints/Loot/LootSource.DropLoot` _returnvalue (`self.HeldWeapon`))
  (`self.K2_DestroyActor` _returnvalue)
  (`self.K2_DestroyActor`))

(event `self.ReceiveDestroyed`
  ;[1 1 1] Drop loot on destroy
  (`self.HostDropLoot`)
  (bind _asarena_game_state (cast `/Game/Blueprints/Modes_States_Instances/ArenaGameState` (`GameplayStatics.GetGameState`)))
  (`/Game/Blueprints/Modes_States_Instances/ArenaGameState.HostUpdateEnemiesList` _asarena_game_state self))

(fn `GenerateWeapon`)

(fn `GetClosestPlayer`
  (returns (Closest :type "Pawn Object Reference"))
  (locals (ClosestDistance :type "Float (double-precision)" :default 90000000.0))
  (bind _outactors (`GameplayStatics.GetAllActorsOfClass` "/Game/Characters/Player/Blueprints/ThirdPersonCharacter.ThirdPersonCharacter_C"))
  (for _array_element _outactors
    (bind _returnvalue (`KismetMathLibrary.Vector_Distance` (`self.K2_GetActorLocation` _array_element) (`self.K2_GetActorLocation`)))
    (if (<= _returnvalue (`local.ClosestDistance`))
      (set `local.ClosestDistance` _returnvalue)
      (set `self.Closest Player` _array_element)))
  (return (`self.Closest Player`)))

(fn `UpdateWalkSpeed`
  (params (NewWalkSpeed :type "Float (double-precision)"))
  (set `CharacterMovementComponent.MaxWalkSpeed` NewWalkSpeed (`self.CharacterMovement`)))

(fn `UserConstructionScript`)