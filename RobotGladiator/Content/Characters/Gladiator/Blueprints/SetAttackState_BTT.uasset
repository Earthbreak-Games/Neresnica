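; Behavior tree task that sets the Gladiator AI's attack mode based on its distance to the target.
; It measures from the pawn to the TargetLocation blackboard vector and picks one of two attack modes, depending on whether that falls within a fixed range.
; The chosen mode is stored on the GladiatorController and mirrored to the AttackMode blackboard key.
; The task fails if the owner is not a GladiatorController.
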(event `self.ReceiveExecuteAI`
  (params (OwnerController :type "AIController Object Reference") (ControlledPawn :type "Pawn Object Reference"))
  (bind _asgladiator_controller (cast `/Game/Characters/Gladiator/Blueprints/GladiatorController` OwnerController)
    (:`then`
      (if (<= (`KismetMathLibrary.Vector_Distance` (`BlackboardComponent.GetValueAsVector` (`AIBlueprintHelperLibrary.GetBlackboard` OwnerController) "TargetLocation") (`Actor.K2_GetActorLocation` ControlledPawn)) 300.0)
        (bind _output_get (set `/Game/Characters/Gladiator/Blueprints/GladiatorController.CurrentAttackMode` "NewEnumerator0" _asgladiator_controller))
        (bind _returnvalue (`AIBlueprintHelperLibrary.GetBlackboard` _asgladiator_controller))
        (`BlackboardComponent.SetValueAsEnum` _returnvalue "AttackMode" _output_get)
        (else
          (bind _output_get_2 (set `/Game/Characters/Gladiator/Blueprints/GladiatorController.CurrentAttackMode` "NewEnumerator1" _asgladiator_controller))
          (`BlackboardComponent.SetValueAsEnum` _returnvalue "AttackMode" _output_get_2)))
      (`self.FinishExecute` true))
    (:`CastFailed`
      (`self.FinishExecute` false))))