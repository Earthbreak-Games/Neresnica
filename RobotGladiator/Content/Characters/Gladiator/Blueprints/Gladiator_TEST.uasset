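; Test variant of the Gladiator robot enemy character, with health scaled by player count and the current arena round.
; FireMissile spawns a rocket at an arrow component and is meant to home it on a random non-spectating player's pawn.
; The targeting loop is gated on TargetFound, which BeginPlay sets false and nothing here sets true, and it rolls separate random indices for check and target.
; A helper function sets walk speed.
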(event `self.ReceiveBeginPlay`
  (bind _returnvalue (`GameplayStatics.GetGameState`))
  (set `self.TargetFound` false)
  (bind _asarena_game_state (cast `/Game/Blueprints/Modes_States_Instances/ArenaGameState` _returnvalue))
  (set `self.mHealth` (`KismetMathLibrary.Conv_IntToDouble` (* (+ (* (`KismetArrayLibrary.Array_Length` (`GameStateBase.PlayerArray` _returnvalue)) 50) 100) (`/Game/Blueprints/Modes_States_Instances/ArenaGameState.RoundNum` _asarena_game_state)))))

(event `FireMissile`
  (bind _returnvalue (`|SpawnActorFromClass` "/Game/Characters/Gladiator/Blueprints/RocketProjectile.RocketProjectile_C" (`SceneComponent.K2_GetComponentToWorld` (`self.Arrow1`)) "Undefined" "OverrideRootScale" null null))
  (bind _asbp_robot_gladiator_game_mode (cast `/Game/Blueprints/Modes_States_Instances/BP_RobotGladiatorGameMode` (`GameplayStatics.GetGameMode`)))
  (while (`self.TargetFound`)
    (bind _playercontrollers (`/Game/Blueprints/Modes_States_Instances/BP_RobotGladiatorGameMode.PlayerControllers` _asbp_robot_gladiator_game_mode))
    (bind _output (`|GetArrayItem` _playercontrollers (`KismetMathLibrary.RandomIntegerInRange` 0 (`KismetArrayLibrary.Array_Length` _playercontrollers))))
    (if (not (`/Game/Characters/Player/Blueprints/CharacterController.Spectating` _output))
      (bind _asthird_person_character (cast `/Game/Characters/Player/Blueprints/ThirdPersonCharacter` (`Controller.K2_GetPawn` _output)))
      (`/Game/Characters/Gladiator/Blueprints/RocketProjectile.HomingMissle` _returnvalue _asthird_person_character))))

(fn `UpdateWalkSpeed`
  (params (NewWalkSpeed :type "Float (double-precision)"))
  (set `CharacterMovementComponent.MaxWalkSpeed` NewWalkSpeed (`self.CharacterMovement`)))

(fn `UserConstructionScript`)