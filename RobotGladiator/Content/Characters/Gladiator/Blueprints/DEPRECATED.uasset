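; Deprecated Gladiator boss enemy character that starts with test health of 50 and drops boss loot when destroyed.
; Destruction spawns a LootSource carrying a Weak Axe through a Host-to-Client event pair, then updates the ArenaGameState enemy list.
; Damage uses the same relay, but melee, homing-rocket and state-reset logic is disconnected, leaving those events empty.
; UpdateWalkSpeed ignores its input and zeroes walk speed.
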(event `self.ReceiveBeginPlay`
  ;[1 1 1] TEST
  (set `self.mHealth` 50.0))

(event `self.MeleeAttack`
  ;[1 1 1] Attacks
)

(event `self.ReceiveTick`
  (params (DeltaSeconds :type "Float (single-precision)")))

(event `HostNotifyDealDamage`
  (params (OposingUnit :type "BaseUnit Object Reference") (Damage :type "Float (double-precision)"))
  (`self.ClientDealDamage` OposingUnit Damage))

(event `self.MeleeBox.OnComponentBeginOverlap`
  (params (OverlappedComponent :type "PrimitiveComponent Object Reference") (OtherActor :type "Actor Object Reference") (OtherComp :type "PrimitiveComponent Object Reference") (OtherBodyIndex :type Integer) (bFromSweep :type Boolean) (SweepResult :type "HitResult Structure (by ref)")))

(event `ClientDealDamage`
  (params (OposingUnit :type "BaseUnit Object Reference") (Damage :type "Float (double-precision)"))
  (`self.DealDamage` OposingUnit Damage))

(event `ResetState`)

(event `ShootProjectile`)

(event `HostDropLoot`
  (`self.ClientDropLoot`))

(event `ClientDropLoot`
  (bind (_returnvalue_location _returnvalue_rotation) (`KismetMathLibrary.BreakTransform` (`self.GetTransform`)))
  ;[1 1 1] Drop Loot
  (bind _returnvalue (`|SpawnActorFromClass` "/Game/Blueprints/Loot/LootSource.LootSource_C" (`KismetMathLibrary.MakeTransform` _returnvalue_location _returnvalue_rotation) "Undefined" "OverrideRootScale" null null))
  (set `/Game/Blueprints/Loot/LootSource.EnemyType` "BOSS" _returnvalue)
  (set `/Game/Blueprints/Loot/LootSource.BossWeapon` "Weak Axe" _returnvalue)
  (`/Game/Blueprints/Loot/LootSource.DropLoot` _returnvalue)
  (`self.K2_DestroyActor`))

(event `self.ReceiveDestroyed`
  ;[1 1 1] Drop loot on destroy
  (`self.HostDropLoot`)
  (bind _asarena_game_state (cast `/Game/Blueprints/Modes_States_Instances/ArenaGameState` (`GameplayStatics.GetGameState`)))
  (`/Game/Blueprints/Modes_States_Instances/ArenaGameState.HostUpdateEnemiesList` _asarena_game_state self))

(fn `UpdateWalkSpeed`
  (params (`New Max Speed` :type "Float (double-precision)"))
  (set `CharacterMovementComponent.MaxWalkSpeed` 0.0 (`self.CharacterMovement`)))

(fn `UserConstructionScript`)