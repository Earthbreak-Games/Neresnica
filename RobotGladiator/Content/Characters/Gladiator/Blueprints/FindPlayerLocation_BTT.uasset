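; Behavior Tree task that gives a Gladiator AI the location of its nearest player.
; It asks the controlled Gladiator pawn for the closest player, writes that actor's location to a target-location blackboard key, and stores the player as the controller's current target.
; It finishes successfully once both are set, and fails if the casts fail or no valid player is found.
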(event `self.ReceiveExecuteAI`
  (params (OwnerController :type "AIController Object Reference") (ControlledPawn :type "Pawn Object Reference"))
  (bind _asgladiator_bp (cast `/Game/Characters/Gladiator/Blueprints/GladiatorBP` ControlledPawn)
    (:`then`
      (bind _closest (`/Game/Characters/Gladiator/Blueprints/GladiatorBP.GetClosestPlayer` _asgladiator_bp))
      (`/Engine/EditorBlueprintResources/StandardMacros.IsValid` _closest
        (:`Is Valid`
          (`BTFunctionLibrary.SetBlackboardValueAsVector` (`self.BB_TargetLoc`) (`Actor.K2_GetActorLocation` _closest))
          (bind _asgladiator_controller (cast `/Game/Characters/Gladiator/Blueprints/GladiatorController` OwnerController)
            (:`then`
              (set `/Game/Characters/Gladiator/Blueprints/GladiatorController.CurrentTarget` _closest _asgladiator_controller)
              (`self.FinishExecute` true))
            (:`CastFailed`
              (`self.FinishExecute` false))))
        (:`Is Not Valid`
          (`self.FinishExecute` false :!label _label))))
    (:`CastFailed`
      (goto _label))))