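; RocketProjectile is a Gladiator rocket actor that can home in on a target and damage characters it overlaps.
; HomingMissle sets the target's capsule as the ProjectileMovement homing component, then applies a very high homing acceleration after a short delay.
; On any overlap it destroys itself, then calls HostNotifyDealDamage on an overlapped ThirdPersonCharacter with fixed damage, passing that same character as OposingUnit.
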(event `self.ReceiveActorBeginOverlap`
  (params (OtherActor :type "Actor Object Reference"))
  (`self.K2_DestroyActor`)
  (bind _asthird_person_character (cast `/Game/Characters/Player/Blueprints/ThirdPersonCharacter` OtherActor))
  (`/Game/Characters/Player/Blueprints/ThirdPersonCharacter.HostNotifyDealDamage` _asthird_person_character _asthird_person_character 10.0))

(event `HomingMissle`
  (params (TargetToHit :type "/Game/Characters/Player/Blueprints/ThirdPersonCharacter Object Reference"))
  (bind _projectilemovement (`self.ProjectileMovement`))
  (if (`KismetSystemLibrary.IsValid` TargetToHit)
    (set `ProjectileMovementComponent.HomingTargetComponent` (`Character.CapsuleComponent` TargetToHit) _projectilemovement)
    (set `ProjectileMovementComponent.bIsHomingProjectile` true _projectilemovement)
    (`KismetSystemLibrary.Delay` 0.5)
    (set `ProjectileMovementComponent.HomingAccelerationMagnitude` 2500000.0 _projectilemovement)))

(fn `UserConstructionScript`)