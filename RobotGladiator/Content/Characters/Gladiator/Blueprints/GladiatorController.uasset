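; AI controller for the Gladiator character that runs its behavior tree and relays melee and ranged attacks to the pawn.
; BeginPlay and Possess share setup that caches the pawn, stores the closest player as target and writes GladiatorState to the Blackboard.
; A looping timer periodically switches that state through AttackTarget, while separate events forward the attack calls.
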(event `self.ReceiveBeginPlay`
  (bind _asgladiator_bp (cast `/Game/Characters/Gladiator/Blueprints/GladiatorBP` (`self.K2_GetPawn`) :!label _label))
  (set `self.GladiatorPawn` _asgladiator_bp)
  (`self.RunBehaviorTree` "/Game/Characters/Gladiator/Blueprints/GladiatorBT.GladiatorBT")
  (bind _closest (`/Game/Characters/Gladiator/Blueprints/GladiatorBP.GetClosestPlayer` (`self.GladiatorPawn`)))
  (set `self.CurrentTarget` _closest)
  (`BlackboardComponent.SetValueAsEnum` (`AIBlueprintHelperLibrary.GetBlackboard` null) "GladiatorState" (`self.CurrentState`))
  (`KismetSystemLibrary.K2_SetTimerDelegate` (delegate `AttackTarget`) 4.0 true))

(event `self.ReceivePossess`
  (params (PossessedPawn :type "Pawn Object Reference"))
  (goto _label))

(event `AttackTarget`
  (bind _output_get (set `self.CurrentState` "NewEnumerator1"))
  (`BlackboardComponent.SetValueAsEnum` (`AIBlueprintHelperLibrary.GetBlackboard` null) "GladiatorState" _output_get))

(event `GladiatorMeleAttack`
  (`/Game/Characters/Gladiator/Blueprints/GladiatorBP.MeleeAttack` (`self.GladiatorPawn`)))

(event `GladiatorRangedAttack`
  (`/Game/Characters/Gladiator/Blueprints/GladiatorBP.RangedAttack` (`self.GladiatorPawn`)))

(fn `UserConstructionScript`)