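; Gladiator enemy character with melee and ranged attacks that drops boss-type loot when destroyed.
; Attack events set state flags and stop movement; the melee box damages ThirdPersonCharacters on overlap during melee, and ResetState clears the flags and starts cooldown.
; ShootProjectile fires a homing rocket at the target.
; A Movement function chases the target until melee range, but its EventGraph call is disconnected, and BeginPlay sets test health.
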(event `self.ReceiveBeginPlay`
  ;[1 1 1] TEST
  (set `self.mHealth` 50.0))

(event `self.ReceiveTick`
  (params (DeltaSeconds :type "Float (single-precision)")))

(event `self.MeleeAttack`
  ;[1 1 1] No touchie!
  (set `self.mIsAttacking` true)
  (set `self.isMeleeAttack` true)
  (`KismetSystemLibrary.PrintString` "Melee")
  (`NavMovementComponent.StopActiveMovement` (`self.CharacterMovement`)))

(event `self.RangedAttack`
  ;[1 1 1] No touchie!
  (set `self.mIsAttacking` true)
  (set `self.isRangedAttack` true)
  (`KismetSystemLibrary.PrintString` "ranged")
  (`NavMovementComponent.StopActiveMovement` (`self.CharacterMovement`)))

(event `self.MeleeBox.OnComponentBeginOverlap`
  (params (OverlappedComponent :type "PrimitiveComponent Object Reference") (OtherActor :type "Actor Object Reference") (OtherComp :type "PrimitiveComponent Object Reference") (OtherBodyIndex :type Integer) (bFromSweep :type Boolean) (SweepResult :type "HitResult Structure (by ref)"))
  (if (`self.mIsAttacking`)
    (if (`self.isMeleeAttack`)
      (bind _asthird_person_character (cast `/Game/Characters/Player/Blueprints/ThirdPersonCharacter` OtherActor)
        (:`then`
          (`self.DealDamage` _asthird_person_character 10.0)
          (`KismetSystemLibrary.PrintString` (`KismetStringLibrary.Conv_DoubleToString` (`BaseUnit.mHealth` _asthird_person_character))))
        (:`CastFailed`
          (`KismetSystemLibrary.PrintString` "not a player"))))))

(event `ResetState`
  (set `self.mIsAttacking` false)
  (set `self.isMeleeAttack` false)
  (set `self.isRangedAttack` false)
  (set `self.mIsOnCooldown` true))

(event `ShootProjectile`
  (bind _returnvalue (`|SpawnActorFromClass` "/Game/Characters/Gladiator/Blueprints/RocketProjectile.RocketProjectile_C" (`SceneComponent.K2_GetComponentToWorld` (`self.Arrow1`)) "Undefined" "OverrideRootScale" null null))
  (bind _asthird_person_character (cast `/Game/Characters/Player/Blueprints/ThirdPersonCharacter` (`self.mpTarget`))
    (:`then`
      (`/Game/Characters/Gladiator/Blueprints/RocketProjectile.HomingMissle` _returnvalue _asthird_person_character))
    (:`CastFailed`
      (`KismetSystemLibrary.PrintString` "Not static mesh actor!"))))

(event `ClientDropLoot`
  (bind (_returnvalue_location _returnvalue_rotation) (`KismetMathLibrary.BreakTransform` (`self.GetTransform`)))
  ;[1 1 1] Drop Loot
  (bind _returnvalue (`|SpawnActorFromClass` "/Game/Blueprints/Loot/LootSourceTest.LootSourceTest_C" (`KismetMathLibrary.MakeTransform` _returnvalue_location _returnvalue_rotation) "Undefined" "OverrideRootScale" null null))
  (set `/Game/Blueprints/Loot/LootSourceTest.EnemyType` "BOSS" _returnvalue)
  (set `/Game/Blueprints/Loot/LootSourceTest.BossWeapon` "Weak Axe" _returnvalue)
  (`/Game/Blueprints/Loot/LootSourceTest.DropLoot` _returnvalue)
  (`self.K2_DestroyActor`))

(event `self.ReceiveDestroyed`
  ;[1 1 1] Drop loot on destroy
  (`self.ClientDropLoot`))

(fn `Movement`
  (if (`self.mIsAttacking`)
    (`NavMovementComponent.StopActiveMovement` (`self.CharacterMovement`) :!label _label)
    (elif (<= (`self.mDistanceToTarget`) (`self.mMeleeRange`))
      (goto _label)
      (else
        (`AIBlueprintHelperLibrary.SimpleMoveToActor` (`self.GetController` self) (`self.mpTarget`)))))
  (return))

(fn `UserConstructionScript`)