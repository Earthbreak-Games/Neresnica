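; Player controller for a multiplayer arena game that manages each player's lobby interface and respawns spectating players as a new ThirdPersonCharacter.
; Tick refreshes the lobby HUD until ArenaGameState reports game start, then hides it.
; Host events pass button style, background color and ready choices to ArenaGameState, while RepNotifies on player index, choices and HUD flag update local UI and state.
; The possession-time lobby setup is disconnected and never runs.
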(event `Respawn`
  (params (SpawnLoc :type "Vector Structure"))
  ;[1 1 1] Respawn Player
  (if (`self.Spectating`)
    (bind _returnvalue (`|SpawnActorFromClass` "/Game/Characters/Player/Blueprints/ThirdPersonCharacter.ThirdPersonCharacter_C" (`KismetMathLibrary.MakeTransform` SpawnLoc) "Undefined" "OverrideRootScale" null null))
    (`self.K2_SetActorLocation` _returnvalue SpawnLoc false false)
    (`self.Possess` _returnvalue)
    (set `self.Spectating` false)
    (bind _asthird_person_character (cast `/Game/Characters/Player/Blueprints/ThirdPersonCharacter` (`self.K2_GetPawn`)))
    (`/Game/Characters/Player/Blueprints/ThirdPersonCharacter.HostSetSteamName` _asthird_person_character (`PlayerState.GetPlayerName` (`self.PlayerState`)))))

(event `self.ReceiveTick`
  (params (DeltaSeconds :type "Float (single-precision)"))
  ;[1 1 1] Update lobby HUD
  (bind _asarena_game_state (cast `/Game/Blueprints/Modes_States_Instances/ArenaGameState` (`GameplayStatics.GetGameState`)))
  (if (`/Game/Blueprints/Modes_States_Instances/ArenaGameState.GameStarted` _asarena_game_state)
    ;[1 1 1] Hide lobby hud if game started
    (`/Engine/EditorBlueprintResources/StandardMacros.DoOnce` false
      (:`Completed`
        (`self.ClientHideLobbyHUD`)))
    (else
      (`self.ClientUpdateLobbyHUD`))))

(event `self.ReceivePossess`
  (params (PossessedPawn :type "Pawn Object Reference")))

(event `ShowStartButton`
  ;[1 1 1] Show start button on the host
  (bind _asthird_person_character (cast `/Game/Characters/Player/Blueprints/ThirdPersonCharacter` (`self.K2_GetPawn`)))
  (`Widget.SetVisibility` (`/Game/Blueprints/Widgets/Lobby/LobbyHUD.StartButton` (`/Game/Characters/Player/Blueprints/ThirdPersonCharacter.LobbyHUDWidget` _asthird_person_character)) "Visible"))

(event `/Game/Characters/Player/Blueprints/CharacterControllerInterface.ResetViewTarget`
  (`self.SetViewTargetWithBlend` (`GameplayStatics.GetPlayerCharacter` 0)))

(event `HostSetPlayerIndex`
  (params (Index :type Integer))
  ;[1 1 1] Set player index
  (set `self.PlayerIndex` Index))

(event `ClientSetUIInputMode`
  ;[1 1 1] Set input mode to UI only
  (`WidgetBlueprintLibrary.SetInputMode_UIOnlyEx` self null)
  (set `self.bShowMouseCursor` true))

(event `HostAddChosenButtonStyle`
  (params (Style :type "ButtonStyle Structure"))
  ;[1 1 1] Add chosen button style to host list
  (bind _asarena_game_state (cast `/Game/Blueprints/Modes_States_Instances/ArenaGameState` (`GameplayStatics.GetGameState`)))
  (`/Game/Blueprints/Modes_States_Instances/ArenaGameState.AddChosenButtonStyle` _asarena_game_state (`self.PlayerIndex`) Style)
  (set `self.StatChoiceUpdated` true))

(event `HostIncrementReadyPlayer`
  ;[1 1 1] Increment ready players on the host
  (bind _asarena_game_state (cast `/Game/Blueprints/Modes_States_Instances/ArenaGameState` (`GameplayStatics.GetGameState`)))
  (`/Game/Blueprints/Modes_States_Instances/ArenaGameState.IncrementReadyPlayers` _asarena_game_state))

(event `ClientUpdateLobbyHUD`
  ;[1 1 1] Update local lobby HUD
  (bind _asarena_game_state (cast `/Game/Blueprints/Modes_States_Instances/ArenaGameState` (`GameplayStatics.GetGameState`)))
  (`/Game/Blueprints/Modes_States_Instances/ArenaGameState.UpdateLocalLobbyHUD` _asarena_game_state))

(event `HostAddChosenBGColor`
  (params (Color :type "LinearColor Structure"))
  ;[1 1 1] Add chosen background color to host list
  (bind _asarena_game_state (cast `/Game/Blueprints/Modes_States_Instances/ArenaGameState` (`GameplayStatics.GetGameState`)))
  (`/Game/Blueprints/Modes_States_Instances/ArenaGameState.AddChosenBGColor` _asarena_game_state (`self.PlayerIndex`) Color)
  (set `self.StatChoiceUpdated` true))

(event `ClientHideLobbyHUD`
  ;[1 1 1] Hide lobby HUD
  (bind _asthird_person_character (cast `/Game/Characters/Player/Blueprints/ThirdPersonCharacter` (`self.K2_GetPawn`)))
  (bind _lobbyhudwidget (`/Game/Characters/Player/Blueprints/ThirdPersonCharacter.LobbyHUDWidget` _asthird_person_character))
  (`/Engine/EditorBlueprintResources/StandardMacros.IsValid` _lobbyhudwidget
    (:`Is Valid`
      (`Widget.SetVisibility` (`/Game/Blueprints/Widgets/Lobby/LobbyHUD.HUD` _lobbyhudwidget) "Hidden")
      (`Widget.SetVisibility` (`WidgetComponent.GetWidget` (`/Game/Characters/Player/Blueprints/ThirdPersonCharacter.StatSelect` _asthird_person_character)) "Hidden")
      ;[1 1 1] Start End lobby sequence
      (bind _asarena_game_state (cast `/Game/Blueprints/Modes_States_Instances/ArenaGameState` (`GameplayStatics.GetGameState`)))
      (set `/Game/Blueprints/Modes_States_Instances/ArenaGameState.GameStarted` true _asarena_game_state)
      (set `self.bShowMouseCursor` false))))

(event `HostHideLobbyHUD`
  ;[1 1 1] Server notify hide lobby HUD
  (set `self.HideHUD` true))

(fn `GetPlayerIndex`
  (returns (Index :type Integer))
  ;[1 1 1] Get the player's index
  (return (`self.PlayerIndex`)))

(fn `GetPlayerSteamID`
  (returns (SteamID :type Text))
  ;[1 1 1] Get Steam ID
  (return (`KismetTextLibrary.Conv_StringToText` (`self.SteamPlayerID`))))

(fn `Move to Start Postion`
  (params (Index :type Integer))
  ;[1 1 1] Move player to start point based on player index
  (bind _asarena_game_state (cast `/Game/Blueprints/Modes_States_Instances/ArenaGameState` (`GameplayStatics.GetGameState`)))
  (`AIBlueprintHelperLibrary.SimpleMoveToLocation` self (`|GetArrayItem` (`/Game/Blueprints/Level/PlayerStartPoints.Points` (`/Game/Blueprints/Modes_States_Instances/ArenaGameState.StartPoints` _asarena_game_state)) Index)))

(fn `OnRep_HideHUD`
  ;[1 1 1] Set game started
  (bind _asarena_game_state (cast `/Game/Blueprints/Modes_States_Instances/ArenaGameState` (`GameplayStatics.GetGameState`)))
  (set `/Game/Blueprints/Modes_States_Instances/ArenaGameState.GameStarted` true _asarena_game_state))

(fn `OnRep_PlayerIndex`
  ;[1 1 1] Show and init lobby UI
  (bind _asthird_person_character (cast `/Game/Characters/Player/Blueprints/ThirdPersonCharacter` (`GameplayStatics.GetPlayerCharacter` 0)))
  (`/Game/Characters/Player/Blueprints/ThirdPersonCharacter.ClientDisplayLobbyUI` _asthird_person_character)
  (`/Game/Characters/Player/Blueprints/ThirdPersonCharacter.ClientInitLobbyHUD` _asthird_person_character))

(fn `OnRep_StatChoiceUpdated`
  ;[1 1 1] Update local HUD
  (`self.ClientUpdateLobbyHUD`))

(fn `UserConstructionScript`)