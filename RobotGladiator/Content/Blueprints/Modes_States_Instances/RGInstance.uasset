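; RGInstance is a game instance Blueprint that manages the multiplayer session lifecycle for the game.
; HostSession creates an advanced session tagged with a server name and player limit, while JoinSession joins a given search result, and each sets IsHosting on success.
; Shutdown and DestroyServer share one path that destroys the session.
; Results are only printed as debug strings, and the network error handler is empty.
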(event `HostSession`
  (params (SName :type String))
  (`CreateSessionCallbackProxyAdvanced.CreateAdvancedSession` (`|MakeArray` (`AdvancedSessionsLibrary.MakeLiteralSessionPropertyString` "SNAME" SName)) (`GameplayStatics.GetPlayerController` 0) (`self.MaxPlayers`)
    (:`then`
      (`KismetSystemLibrary.PrintString` "Finished"))
    (:`OnSuccess`
      (`KismetSystemLibrary.PrintString` "Created session")
      (set `self.bIsHosting` true))
    (:`OnFailure`
      (`KismetSystemLibrary.PrintString` "Failed to create session"))))

(event `JoinSession`
  (params (SessionResult :type "BlueprintSessionResult Structure"))
  (`JoinSessionCallbackProxy.JoinSession` (`GameplayStatics.GetPlayerController` 0) SessionResult
    (:`OnSuccess`
      (`KismetSystemLibrary.PrintString` "Joined session")
      (set `self.bIsHosting` false))
    (:`OnFailure`
      (`KismetSystemLibrary.PrintString` "Failed to join session"))))

(event `self.HandleNetworkError`
  (params (FailureType :type "ENetworkFailure Enum" :default "NetDriverAlreadyExists") (bIsServer :type Boolean)))

(event `self.ReceiveShutdown`
  (`DestroySessionCallbackProxy.DestroySession` (`GameplayStatics.GetPlayerController` 0) :!label _label
    (:`OnSuccess`
      (`KismetSystemLibrary.PrintString` "Destroyed session"))
    (:`OnFailure`
      (`KismetSystemLibrary.PrintString` "Failed to destroy session"))))

(event `DestroyServer`
  (goto _label))