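; Player state for the robot gladiator arena that puts a player into spectate mode.
; StartSpectating passes a player ID to HostSetSpectateView, which searches the BP_RobotGladiatorGameMode controller list and calls Spectate on the controller with that ID.
; The lookup depends on the game mode cast succeeding, and GetPlayerIndex is a stub that always returns zero.
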(event `HostSetSpectateView`
  (params (PlayerStateID :type Integer))
  (bind _asbp_robot_gladiator_game_mode (cast `/Game/Blueprints/Modes_States_Instances/BP_RobotGladiatorGameMode` (`GameplayStatics.GetGameMode`)))
  (for _array_element (`/Game/Blueprints/Modes_States_Instances/BP_RobotGladiatorGameMode.PlayerControllers` _asbp_robot_gladiator_game_mode)
    (if (== (`PlayerState.PlayerId` (`Controller.PlayerState` _array_element)) PlayerStateID)
      (`ArenaPlayerController.Spectate` _array_element))))

(event `/Game/Blueprints/Modes_States_Instances/ArenaPlayerStateInterface.StartSpectating`
  (params (PlayerStateID :type Integer))
  (`self.HostSetSpectateView` PlayerStateID))

(fn `GetPlayerIndex`
  (returns (Index :type Integer))
  (return 0))

(fn `UserConstructionScript`)