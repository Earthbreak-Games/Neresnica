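; Game state for a multiplayer robot gladiator arena, tracking lobby readiness and style choices, round number, living enemies and player deaths.
; Four ready players reveal the start button, then a timed camera sequence moves players to start points and starts a round.
; Round changes iterate the LobbySpawns Grid level, respawn players and rebuild the enemy list.
; Clearing enemies ends the round; all players dead flags game over.
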(event `self.ReceiveBeginPlay`
  ;[1 1 1] Init button and color arrays for lobby HUD
  (for _ (range 4)
    (`KismetArrayLibrary.Array_Add` (`self.ChosenButtonStyles`) (`self.DefaultStyle`))
    (`KismetArrayLibrary.Array_Add` (`self.ChosenBGColors`) (`self.DefaultColor`))))

(event `PlayerJoined`
  ;[1 1 1] Player Joined Game
  (`/Engine/EditorBlueprintResources/ActorMacros.Switch Has Authority`
    (:`Authority`
      (bind _asbp_robot_gladiator_game_mode (cast `/Game/Blueprints/Modes_States_Instances/BP_RobotGladiatorGameMode` (`GameplayStatics.GetGameMode`)))
      (`/Engine/EditorBlueprintResources/StandardMacros.IsValid` (`self.LobbySpawns`)
        (:`Is Valid`
          _)
        (:`Is Not Valid`
          (bind _outactors (`GameplayStatics.GetAllActorsOfClass` "/Game/Blueprints/Level/LobbySpawnPoints.LobbySpawnPoints_C"))
          (set `self.LobbySpawns` (`|GetArrayItem` _outactors))))
      (`/Game/Blueprints/Level/LobbySpawnPoints.SetSpawnPositions` (`self.LobbySpawns`) (`/Game/Blueprints/Modes_States_Instances/BP_RobotGladiatorGameMode.PlayerControllers` _asbp_robot_gladiator_game_mode))
      (`/Engine/EditorBlueprintResources/StandardMacros.IsValid` (`self.StartPoints`)
        (:`Is Not Valid`
          (bind _outactors_2 (`GameplayStatics.GetAllActorsOfClass` "/Game/Blueprints/Level/PlayerStartPoints.PlayerStartPoints_C"))
          (set `self.StartPoints` (`|GetArrayItem` _outactors_2)))))))

(event `UpdateLocalLobbyHUD`
  ;[1 1 1] Update local client's lobby HUD
  (bind _asthird_person_character (cast `/Game/Characters/Player/Blueprints/ThirdPersonCharacter` (`Controller.K2_GetPawn` (`GameplayStatics.GetPlayerController` 0))))
  (bind _lobbyhudwidget (`/Game/Characters/Player/Blueprints/ThirdPersonCharacter.LobbyHUDWidget` _asthird_person_character))
  (`/Engine/EditorBlueprintResources/StandardMacros.IsValid` _lobbyhudwidget
    (:`Is Valid`
      (`/Game/Blueprints/Widgets/Lobby/LobbyHUD.UpdateLobbyHUD` _lobbyhudwidget))))

(event `UpdateLocalGameOverScreen`
  (bind _ascharacter_controller (cast `/Game/Characters/Player/Blueprints/CharacterController` (`GameplayStatics.GetPlayerController` 0)))
  (bind _endscreenwidget (`/Game/Characters/Player/Blueprints/CharacterController.EndScreenWidget` _ascharacter_controller))
  (`/Engine/EditorBlueprintResources/StandardMacros.IsValid` _endscreenwidget
    (:`Is Valid`
      (`/Game/Blueprints/Widgets/InGameMenus/GameOverScreen.SetScreenInfo` _endscreenwidget))
    (:`Is Not Valid`
      (bind _returnvalue (`|CreateWidget` "/Game/Blueprints/Widgets/InGameMenus/GameOverScreen.GameOverScreen_C"))
      (bind _output_get (set `/Game/Characters/Player/Blueprints/CharacterController.EndScreenWidget` _returnvalue _ascharacter_controller))
      (`/Engine/EditorBlueprintResources/StandardMacros.IsValid` _output_get
        (:`Is Valid`
          (`UserWidget.AddToViewport` _output_get 0)
          (`/Game/Blueprints/Widgets/InGameMenus/GameOverScreen.SetScreenInfo` _output_get))))))

(event `AddChosenButtonStyle`
  (params (Index :type Integer) (Style :type "ButtonStyle Structure"))
  ;[1 1 1] Set Chosen Button Style
  (`KismetArrayLibrary.Array_Set` (`self.ChosenButtonStyles`) Index Style))

(event `AddChosenBGColor`
  (params (Index :type Integer) (Color :type "LinearColor Structure"))
  ;[1 1 1] Set Chosen BG Color
  (`KismetArrayLibrary.Array_Set` (`self.ChosenBGColors`) Index Color))

(event `IncrementReadyPlayers`
  ;[1 1 1] Increment number of ready players
  (set `self.NumReadyPlayers` (+ (`self.NumReadyPlayers`) 1))
  ;[1 1 1] Show Start Button if all players are ready
  (if (>= (`self.NumReadyPlayers`) 4)
    (bind _ascharacter_controller (cast `/Game/Characters/Player/Blueprints/CharacterController` (`GameplayStatics.GetPlayerController` 0)))
    (`/Game/Characters/Player/Blueprints/CharacterController.ShowStartButton` _ascharacter_controller)))

(event `/Game/Blueprints/Modes_States_Instances/ArenaGameStateInterface.MoveLobbyCamera`
  (params (Move :type Boolean))
  ;[1 1 1] Move lobby cameras
  (`self.HostNotifyLobbyCameraMove` Move))

(event `ChangeRound`
  (bind _grid (`/Game/Blueprints/Level/LobbySpawnPoints.Grid` (`self.LobbySpawns`)))
  ;[1 1 1] Handle Round Changes
  (`/Game/Blueprints/Level/BPArenaGrid.Iterate_Level` _grid)
  (`self.Increment Round`)
  (`self.RespawnPlayers`)
  (`KismetSystemLibrary.Delay` 5.0)
  (`/Game/Blueprints/Level/BPArenaGrid.Begin_Round` _grid)
  (`self.ResetEnemyArrays`))

(event `HostNotifyLobbyCameraMove`
  (params (Move :type Boolean))
  ;[1 1 1] Host notify camera movement
  (`self.ClientMoveLobbyCamera` Move)
  (if (not Move)
    (`self.HostMoveToStartPoints`)))

(event `HostChangeRound`
  ;[1 1 1] Host Change Round
  (`self.ChangeRound`))

(event `HostUpdateEnemiesList`
  (params (Gladiator :type "/Game/Characters/Gladiator/Blueprints/Gladiator Object Reference"))
  (bind _gladiators (`self.Gladiators`))
  (bind _lobbyspawns (`self.LobbySpawns`))
  ;[1 1 1] Update list of living enemies
  (`KismetArrayLibrary.Array_RemoveItem` _gladiators Gladiator)
  (`KismetSystemLibrary.PrintString` "Enemy Killed" true true (struct :`R` 1.0 :`G` 0.71853 :`A` 1.0))
  (if (== (`KismetArrayLibrary.Array_Length` _gladiators) 0)
    (`/Engine/EditorBlueprintResources/StandardMacros.IsValid` _lobbyspawns
      (:`Is Valid`
        (`/Game/Blueprints/Level/BPArenaGrid.End_Round` (`/Game/Blueprints/Level/LobbySpawnPoints.Grid` _lobbyspawns))))))

(event `ClientMoveLobbyCamera`
  (params (Move :type Boolean))
  (bind _grid (`/Game/Blueprints/Level/LobbySpawnPoints.Grid` (`self.LobbySpawns`)))
  ;[1 1 1] Client activate camera movement
  (bind _output_get (set `/Game/Blueprints/Level/BPArenaGrid.ExitLobby` Move _grid))
  (if _output_get
    (`/Game/Blueprints/Level/BPArenaGrid.Exit_Lobby` _grid)
    (else
      (`KismetSystemLibrary.Delay` 1.0)
      (set `/Game/Blueprints/Level/BPArenaGrid.EndLobbySequence` true _grid)
      (`KismetSystemLibrary.Delay` 7.0)
      (set `/Game/Blueprints/Level/BPArenaGrid.EndLobbySequence` false _grid)
      (bind _ascharacter_controller (cast `/Game/Characters/Player/Blueprints/CharacterController` (`GameplayStatics.GetPlayerController` 0)))
      (`WidgetBlueprintLibrary.SetInputMode_GameOnly` _ascharacter_controller)
      (`self.HostChangeRound`))))

(event `/Game/Blueprints/Modes_States_Instances/ArenaGameStateInterface.TriggerRoundChange`
  (`self.HostChangeRound`))

(event `HostMoveToStartPoints`
  ;[1 1 1] Move players to their start positions
  (bind _asbp_robot_gladiator_game_mode (cast `/Game/Blueprints/Modes_States_Instances/BP_RobotGladiatorGameMode` (`GameplayStatics.GetGameMode`)))
  (for (_array_element _array_index) (`/Game/Blueprints/Modes_States_Instances/BP_RobotGladiatorGameMode.PlayerControllers` _asbp_robot_gladiator_game_mode)
    (`/Game/Characters/Player/Blueprints/CharacterController.Move to Start Postion` _array_element _array_index))
  (`KismetSystemLibrary.Delay` 1.0)
  (set `/Game/Blueprints/Level/BPArenaGrid.ResetCenterRing` true (`/Game/Blueprints/Level/LobbySpawnPoints.Grid` (`self.LobbySpawns`))))

(event `/Game/Blueprints/Modes_States_Instances/ArenaGameStateInterface.IncrementDeadPlayerCount`
  (`self.HostIncrementDeaths`))

(event `HostIncrementDeaths`
  (set `self.NumDeadPlayers` (+ (`self.NumDeadPlayers`) 1))
  (bind _asbp_robot_gladiator_game_mode (cast `/Game/Blueprints/Modes_States_Instances/BP_RobotGladiatorGameMode` (`GameplayStatics.GetGameMode`)))
  (bind _playercontrollers (`/Game/Blueprints/Modes_States_Instances/BP_RobotGladiatorGameMode.PlayerControllers` _asbp_robot_gladiator_game_mode))
  (if (>= (`self.NumDeadPlayers`) (`KismetArrayLibrary.Array_Length` _playercontrollers))
    (for _array_element _playercontrollers
      (set `/Game/Characters/Player/Blueprints/CharacterController.GameOver` true _array_element))))

(event `/Game/Blueprints/Modes_States_Instances/ArenaGameStateInterface.DecrementDeadPlayerCount`
  (`self.HostDecrementDeaths`))

(event `HostDecrementDeaths`
  (set `self.NumDeadPlayers` (- (`self.NumDeadPlayers`) 1)))

(fn `GetPawnToSpectate`
  (returns (Pawn :type "Pawn Object Reference"))
  (locals (randIndex :type Integer))
  (return null))

(fn `GetPlayerControllersFromGameMode`
  (returns (PlayerControllers :type "Array of /Game/Characters/Player/Blueprints/CharacterController Object Reference"))
  (bind _asbp_robot_gladiator_game_mode (cast `/Game/Blueprints/Modes_States_Instances/BP_RobotGladiatorGameMode` (`GameplayStatics.GetGameMode`)))
  (return (`/Game/Blueprints/Modes_States_Instances/BP_RobotGladiatorGameMode.PlayerControllers` _asbp_robot_gladiator_game_mode)))

(fn `Increment Round`
  (set `self.RoundNum` (+ (`self.RoundNum`) 1))
  (`KismetSystemLibrary.PrintString` (`KismetStringLibrary.Conv_IntToString` (`self.RoundNum`)) true true (struct :`R` 1.0 :`G` 0.03805 :`B` 0.117728 :`A` 1.0)))

(fn `ResetEnemyArrays`
  (`KismetArrayLibrary.Array_Clear` (`self.Gladiators`))
  (bind _outactors (`GameplayStatics.GetAllActorsOfClass` "/Game/Characters/Gladiator/Blueprints/Gladiator.Gladiator_C"))
  (set `self.Gladiators` _outactors))

(fn `RespawnPlayers`
  (bind _asbp_robot_gladiator_game_mode (cast `/Game/Blueprints/Modes_States_Instances/BP_RobotGladiatorGameMode` (`GameplayStatics.GetGameMode`)))
  (for (_array_element _array_index) (`/Game/Blueprints/Modes_States_Instances/BP_RobotGladiatorGameMode.PlayerControllers` _asbp_robot_gladiator_game_mode)
    (`/Game/Characters/Player/Blueprints/CharacterController.Respawn` _array_element (+ (`|GetArrayItem` (`/Game/Blueprints/Level/PlayerStartPoints.Points` (`self.StartPoints`)) _array_index) (0.0 0.0 100.0)))))

(fn `UserConstructionScript`)