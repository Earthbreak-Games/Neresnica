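; Missile actor that picks a ThirdPersonCharacter as its target and destroys itself on any actor overlap.
; Tick calls FindTarget while targeting is enabled and no valid target exists; the Targeting branch for a valid target is empty.
; FindTarget loops over all characters, but its distance check does nothing, so the last element becomes Target.
; Homing is unfinished: the FloatingPawnMovement velocity and speed setters are disconnected.
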(event `self.ReceiveBeginPlay`
  (set `self.shouldTarget` true))

(event `self.ReceiveActorBeginOverlap`
  (params (OtherActor :type "Actor Object Reference"))
  (`self.K2_DestroyActor`))

(event `self.ReceiveTick`
  (params (DeltaSeconds :type "Float (single-precision)"))
  (if (`self.shouldTarget`)
    (if (`KismetSystemLibrary.IsValid` (`self.target`))
      (if (`self.targeting`)
        _)
      (else
        (`self.FindTarget`)))))

(fn `FindTarget`
  (bind _outactors (`GameplayStatics.GetAllActorsOfClass` "/Game/Character/Blueprints/ThirdPersonCharacter.ThirdPersonCharacter_C"))
  (for _array_element _outactors
    (if (> (`self.GetDistanceTo` _array_element self) (`self.distanceToTarget`))
      _))
  (bind _asthird_person_character (cast `/Game/Character/Blueprints/ThirdPersonCharacter` _array_element))
  (set `self.target` _asthird_person_character))

(fn `UserConstructionScript`)