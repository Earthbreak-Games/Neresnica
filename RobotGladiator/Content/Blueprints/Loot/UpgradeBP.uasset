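; UpgradeBP is a ground upgrade pickup that shows a widget while a ThirdPersonCharacter is within its PickUpSphere.
; Sphere overlaps toggle CanPickUp and widget visibility, and set or clear the character's GroundUpgrade reference to this actor.
; Each Tick scales the widget by the player's distance, shrinking it to half size as the player moves away.
; The pickup action itself is not implemented in this Blueprint.
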(event `self.ReceiveTick`
  (params (DeltaSeconds :type "Float (single-precision)"))
  (bind _returnvalue (`GameplayStatics.GetPlayerCharacter` 0))
  (bind _widget (`self.Widget`))
  (bind _returnvalue_2 (`KismetMathLibrary.MapRangeClamped` (`KismetMathLibrary.VSize` (- (`self.K2_GetActorLocation` _returnvalue) (`self.K2_GetActorLocation`))) 50.0 2000.0 1.0 0.5))
  ;[1 1 1] Resize Widget
  (`/Engine/EditorBlueprintResources/StandardMacros.IsValid` _returnvalue
    (:`Is Valid`
      (`/Engine/EditorBlueprintResources/StandardMacros.IsValid` _widget
        (:`Is Valid`
          (`Widget.SetRenderScale` (`WidgetComponent.GetWidget` _widget) (`KismetMathLibrary.MakeVector2D` _returnvalue_2 _returnvalue_2)))))))

(event `self.PickUpSphere.OnComponentBeginOverlap`
  (params (OverlappedComponent :type "PrimitiveComponent Object Reference") (OtherActor :type "Actor Object Reference") (OtherComp :type "PrimitiveComponent Object Reference") (OtherBodyIndex :type Integer) (bFromSweep :type Boolean) (SweepResult :type "HitResult Structure (by ref)"))
  (bind _asthird_person_character (cast `/Game/Characters/Player/Blueprints/ThirdPersonCharacter` OtherActor))
  (set `self.CanPickUp` true)
  (set `/Game/Characters/Player/Blueprints/ThirdPersonCharacter.GroundUpgrade` self _asthird_person_character)
  (`SceneComponent.SetVisibility` (`self.Widget`) true false))

(event `self.PickUpSphere.OnComponentEndOverlap`
  (params (OverlappedComponent :type "PrimitiveComponent Object Reference") (OtherActor :type "Actor Object Reference") (OtherComp :type "PrimitiveComponent Object Reference") (OtherBodyIndex :type Integer))
  (bind _asthird_person_character (cast `/Game/Characters/Player/Blueprints/ThirdPersonCharacter` OtherActor))
  (set `self.CanPickUp` false)
  (set `/Game/Characters/Player/Blueprints/ThirdPersonCharacter.GroundUpgrade` null _asthird_person_character)
  (`SceneComponent.SetVisibility` (`self.Widget`) false false))

(fn `UserConstructionScript`)