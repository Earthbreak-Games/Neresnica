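; Test loot source actor that, on DropLoot, spawns one potential drop per player in a ring around itself.
; LootTable rolls rarity and item type: grunts drop health or rarity-matched data-table armor, while bosses add their own weapon on a Weapon roll to grunt-style extras.
; Pickups get placeholder meshes (armor, weapons), a stats widget, a physics pop and a short lifespan.
; Debug prints remain, and the random weapon branch is disconnected.
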(event `DropLoot`
  (`self.ChooseItem`))

(fn `CalculateLootPosition`
  (params (Index :type Integer))
  (returns (Location :type "Vector Structure"))
  (bind _returnvalue (/ 360.0 (`KismetMathLibrary.Conv_IntToDouble` (`self.NumPlayers`))))
  (return (`KismetMathLibrary.GreaterGreater_VectorRotator` (`KismetMathLibrary.MakeVector` (`self.LootRaduis`)) (`KismetMathLibrary.MakeRotator` 0.0 0.0 (+ (* Index _returnvalue) (`KismetMathLibrary.MapRangeClamped` (`self.LootOffset`) 0.0 1.0 0.0 _returnvalue))))))

(fn `ChooseArmorType`
  (returns (ArmorType :type "EArmorTypes Enum"))
  (return (select `int` (`KismetMathLibrary.RandomIntegerInRange` 0 9) :`0` "HEAD" :`1` "HEAD" :`2` "HEAD" :`3` "HEAD" :`4` "HEAD" :`5` "CHEST" :`6` "CHEST" :`7` "CHEST" :`8` "CHEST" :`9` "CHEST" :!type "EArmorTypes Enum")))

(fn `ChooseItem`
  (locals (CompatibleItems :type "Array of Name") (SelectedRarity :type "ERarities Enum") (SelectedLootType :type "ELootTypes Enum") (LootLocation :type "Vector Structure") (BossWeaponData :type "/Game/Blueprints/Loot/WeaponDataStruct Structure") (ArmorDataList :type "Array of /Game/Blueprints/Loot/ArmorDataStruct Structure") (ArmorData :type "/Game/Blueprints/Loot/ArmorDataStruct Structure") (Rand :type Integer))
  (bind _compatibleitems (`local.CompatibleItems`))
  (bind (_name _rarity _weapontype _basedamage) (break `/Game/Blueprints/Loot/WeaponDataStruct` (`local.BossWeaponData`)))
  (bind (_name_2 _rarity_2 _armortype _defense) (break `/Game/Blueprints/Loot/ArmorDataStruct` (`local.ArmorData`)))
  ;[1 1 1] Choose rarity
  (bind _returnvalue (`LootTable.ChooseRarity` (`self.LootTable`) 0.0))
  (set `local.SelectedRarity` _returnvalue)
  (switch `EEnemyTypes` (`self.EnemyType`)
    (:`GRUNT`
      (for _index (range (`self.NumPlayers`))
        ;[1 1 1] Calculate loot drop position
        (bind _location (`self.CalculateLootPosition` _index))
        (set `local.LootLocation` _location)
        ;[1 1 1] Choose item type based off of enemy
        (bind _returnvalue_2 (`LootTable.ChooseItemType` (`self.LootTable`) (`self.EnemyType`) 0.0))
        (bind _output_get (set `local.SelectedLootType` _returnvalue_2))
        (`KismetSystemLibrary.PrintString` (`|GetEnumeratorNameAsString` _output_get) true true (struct :`R` 0.1305 :`G` 0.063542 :`B` 1.0 :`A` 1.0))
        (switch `ELootTypes` _output_get :!label _label
          (:`HEALTH`
            ;[1 1 1] Drop Health
            (`KismetSystemLibrary.PrintString` "Health")
            (bind _returnvalue_3 (`|SpawnActorFromClass` "/Game/Blueprints/Loot/HealthPickup.HealthPickup_C" (`KismetMathLibrary.MakeTransform` (+ (`self.K2_GetActorLocation`) (`local.LootLocation`))) "Undefined" "OverrideRootScale" null null))
            (bind _asloot_hud_bp (cast `/Game/Blueprints/Loot/LootHUD_BP` (`WidgetComponent.GetUserWidgetObject` (`/Game/Blueprints/Loot/HealthPickup.Widget` _returnvalue_3))))
            (`/Game/Blueprints/Loot/LootHUD_BP.SetBGColors` _asloot_hud_bp "COMMON" true)
            (`/Game/Blueprints/Loot/LootHUD_BP.SetHUDInfo` _asloot_hud_bp "None" "COMMON" "SWORD" "HEAD" 0 true false)
            (bind _sphere (`/Game/Blueprints/Loot/HealthPickup.Sphere` _returnvalue_3))
            (`PrimitiveComponent.SetSimulatePhysics` _sphere true)
            (`PrimitiveComponent.AddImpulse` _sphere (0.0 0.0 250.0) "None" true)
            (`PrimitiveComponent.AddRadialImpulse` _sphere (`self.K2_GetActorLocation`) 500.0 100.0 "RIF_Constant" true)
            (`self.SetLifeSpan` _returnvalue_3 2.0))
          (:`ARMOR`
            ;[1 1 1] Drop Armor
            (bind _armortype_2 (`self.ChooseArmorType`))
            (bind _outrownames (`DataTableFunctionLibrary.GetDataTableRowNames` "/Game/Data/ArmorDataTable.ArmorDataTable"))
            (for _array_element _outrownames
              (bind _returnvalue_4 (`|GetDataTableRow` "/Game/Data/ArmorDataTable.ArmorDataTable" _array_element)
                (:`then`
                  (bind (_name_3 _rarity_3 _armortype_3) (break `/Game/Blueprints/Loot/ArmorDataStruct` _returnvalue_4))
                  (if (and (`|EnumEquality` _rarity_3 (`local.SelectedRarity`)) (`|EnumEquality` _armortype_3 _armortype_2))
                    (`KismetArrayLibrary.Array_Add` (`local.CompatibleItems`) _name_3)
                    (`KismetArrayLibrary.Array_Add` (`local.ArmorDataList`) _returnvalue_4)))))
            (bind _output_get_2 (set `local.Rand` (`KismetMathLibrary.RandomIntegerInRange` 0 (`KismetArrayLibrary.Array_LastIndex` _compatibleitems))))
            (bind _output (`|GetArrayItem` _compatibleitems _output_get_2))
            (if (not (== _output "None"))
              (set `local.ArmorData` (`|GetArrayItem` (`local.ArmorDataList`) _output_get_2))
              (bind _returnvalue_5 (`|SpawnActorFromClass` "/Game/Blueprints/Loot/ArmorBP.ArmorBP_C" (`KismetMathLibrary.MakeTransform` (+ (`self.K2_GetActorLocation`) (`local.LootLocation`))) "AlwaysSpawn" "OverrideRootScale" null _output null))
              (`Armor.SetArmorStats` _returnvalue_5 _defense _rarity_2 _armortype)
              (`self.SelectArmorMesh` (`Armor.Mesh` _returnvalue_5) _rarity_2 _armortype)
              (bind _asloot_hud_bp_2 (cast `/Game/Blueprints/Loot/LootHUD_BP` (`WidgetComponent.GetUserWidgetObject` (`/Game/Blueprints/Loot/ArmorBP.Widget` _returnvalue_5))))
              (`/Game/Blueprints/Loot/LootHUD_BP.SetBGColors` _asloot_hud_bp_2 _rarity_2 false)
              (`/Game/Blueprints/Loot/LootHUD_BP.SetHUDInfo` _asloot_hud_bp_2 _name_2 _rarity_2 "SWORD" _armortype _defense false false)
              (bind _mesh (`Armor.Mesh` _returnvalue_5))
              (`PrimitiveComponent.SetSimulatePhysics` _mesh true)
              (`PrimitiveComponent.AddImpulse` _mesh (0.0 0.0 250.0) "None" true)
              (`PrimitiveComponent.AddRadialImpulse` _mesh (`self.K2_GetActorLocation`) 500.0 100.0 "RIF_Constant" true)
              (`self.SetLifeSpan` _returnvalue_5 2.0)
              (`KismetSystemLibrary.PrintString` (`KismetStringLibrary.Conv_NameToString` _name_2) true true (struct :`R` 0.207391 :`G` 1.0 :`A` 1.0))
              (`KismetSystemLibrary.PrintString` (`|GetEnumeratorNameAsString` _rarity_2))
              (`KismetSystemLibrary.PrintString` (`|GetEnumeratorNameAsString` _armortype) true true (struct :`R` 1.0 :`G` 0.17058 :`A` 1.0)))))))
    (:`BOSS`
      (`|ExecutionSequence`
        (:`then_0`
          (for _index_2 (range 1 (`self.NumPlayers`))
            ;[1 1 1] Calculate loot drop position
            (bind _location_2 (`self.CalculateLootPosition` _index_2))
            (set `local.LootLocation` _location_2)
            ;[1 1 1] Choose additional item type for boss to drop
            (bind _returnvalue_6 (`LootTable.ChooseItemType` (`self.LootTable`) "GRUNT" 0.0))
            (set `local.SelectedLootType` _returnvalue_6)
            (goto _label)))
        (:`then_1`
          ;[1 1 1] Calculate loot drop position
          (bind _location_3 (`self.CalculateLootPosition` 0))
          (set `local.LootLocation` _location_3)
          ;[1 1 1] Choose item type based off of enemy
          (bind _returnvalue_7 (`LootTable.ChooseItemType` (`self.LootTable`) (`self.EnemyType`) 0.0))
          (bind _output_get_3 (set `local.SelectedLootType` _returnvalue_7))
          (`KismetSystemLibrary.PrintString` (`|GetEnumeratorNameAsString` _output_get_3) true true (struct :`R` 0.1305 :`G` 0.063542 :`B` 1.0 :`A` 1.0))
          ;[1 1 1] Drop boss' current weapon
          (switch `ELootTypes` _output_get_3
            (:`WEAPON`
              (bind _outrownames_2 (`DataTableFunctionLibrary.GetDataTableRowNames` "/Game/Data/WeaponDataTable.WeaponDataTable"))
              (for _array_element_2 _outrownames_2
                (bind _returnvalue_8 (`|GetDataTableRow` "/Game/Data/WeaponDataTable.WeaponDataTable" _array_element_2)
                  (:`then`
                    (if (== (`.Name_2_B2B2B0EE4F506D39AB086C9C167C9782` (break `/Game/Blueprints/Loot/WeaponDataStruct` _returnvalue_8)) (`self.BossWeapon`))
                      (set `local.BossWeaponData` _returnvalue_8)
                      (break)))))
              (bind _returnvalue_9 (`|SpawnActorFromClass` "/Game/Blueprints/Loot/WeaponBP.WeaponBP_C" (`KismetMathLibrary.MakeTransform` (+ (`self.K2_GetActorLocation`) (`local.LootLocation`))) "AlwaysSpawn" "OverrideRootScale" null (`self.BossWeapon`) null))
              (`Weapon.SetWeaponStats` _returnvalue_9 _basedamage _rarity _weapontype)
              (bind _mesh_2 (`Weapon.Mesh` _returnvalue_9))
              (`self.SelectWeaponMesh` _mesh_2 _rarity _weapontype)
              (bind _asloot_hud_bp_3 (cast `/Game/Blueprints/Loot/LootHUD_BP` (`WidgetComponent.GetUserWidgetObject` (`/Game/Blueprints/Loot/WeaponBP.Widget` _returnvalue_9))))
              (`/Game/Blueprints/Loot/LootHUD_BP.SetBGColors` _asloot_hud_bp_3 _rarity false)
              (`/Game/Blueprints/Loot/LootHUD_BP.SetHUDInfo` _asloot_hud_bp_3 _name _rarity _weapontype "HEAD" _basedamage false true)
              (`PrimitiveComponent.SetSimulatePhysics` _mesh_2 true)
              (`PrimitiveComponent.AddImpulse` _mesh_2 (0.0 0.0 250.0) "None" true)
              (`PrimitiveComponent.AddRadialImpulse` _mesh_2 (`self.K2_GetActorLocation`) 500.0 100.0 "RIF_Constant" true)
              (`self.SetLifeSpan` _returnvalue_9 2.0)
              (`KismetSystemLibrary.PrintString` (`KismetStringLibrary.Conv_NameToString` _name) true true (struct :`R` 0.070153 :`G` 1.0 :`A` 1.0))
              (`KismetSystemLibrary.PrintString` (`|GetEnumeratorNameAsString` _rarity))
              (`KismetSystemLibrary.PrintString` (`|GetEnumeratorNameAsString` _weapontype) true true (struct :`R` 1.0 :`G` 0.886987 :`A` 1.0)))))))))

(fn `ChooseWeaponType`
  (returns (WeaponType :type "EWeaponTypes Enum"))
  (return (select `int` (`KismetMathLibrary.RandomIntegerInRange` 0 9) :`0` "SWORD" :`1` "SWORD" :`2` "SWORD" :`3` "AXE" :`4` "AXE" :`5` "AXE" :`6` "SHIELD" :`7` "SHIELD" :`8` "SHIELD" :`9` "SWORD" :!type "EWeaponTypes Enum")))

(fn `SelectArmorMesh`
  (params (MeshComponent :type "StaticMeshComponent Object Reference") (Rarity :type "ERarities Enum" :default "COMMON") (ArmorType :type "EArmorTypes Enum" :default "HEAD"))
  (locals (ItemMeshComponent :type "StaticMeshComponent Object Reference"))
  (bind _itemmeshcomponent (`local.ItemMeshComponent`))
  (bind _itemmeshcomponent_2 (`local.ItemMeshComponent`))
  (bind _itemmeshcomponent_3 (`local.ItemMeshComponent`))
  (set `local.ItemMeshComponent` MeshComponent)
  (switch `EArmorTypes` ArmorType
    (:`HEAD`
      (`StaticMeshComponent.SetStaticMesh` _itemmeshcomponent_2 "/Game/Geometry/Meshes/1M_Cube.1M_Cube")
      (`SceneComponent.SetWorldScale3D` _itemmeshcomponent_2 (0.5 0.5 0.5)))
    (:`CHEST`
      (`StaticMeshComponent.SetStaticMesh` (`local.ItemMeshComponent`) "/Game/Geometry/Meshes/1M_Cube.1M_Cube"))
    (:`ARMS`
      (`StaticMeshComponent.SetStaticMesh` _itemmeshcomponent_3 "/Game/Geometry/Meshes/1M_Cube.1M_Cube")
      (`SceneComponent.SetWorldScale3D` _itemmeshcomponent_3 (0.5 0.5 0.25)))
    (:`LEGS`
      (`StaticMeshComponent.SetStaticMesh` _itemmeshcomponent "/Game/Geometry/Meshes/1M_Cube.1M_Cube")
      (`SceneComponent.SetWorldScale3D` _itemmeshcomponent (0.5 0.5 1.0)))))

(fn `SelectWeaponMesh`
  (params (MeshComponent :type "StaticMeshComponent Object Reference") (Rarity :type "ERarities Enum" :default "COMMON") (WeaponType :type "EWeaponTypes Enum" :default "SWORD"))
  (locals (ItemMeshComponent :type "StaticMeshComponent Object Reference"))
  (bind _itemmeshcomponent (`local.ItemMeshComponent`))
  (bind _itemmeshcomponent_2 (`local.ItemMeshComponent`))
  (set `local.ItemMeshComponent` MeshComponent)
  (switch `EWeaponTypes` WeaponType
    (:`SWORD`
      (`StaticMeshComponent.SetStaticMesh` _itemmeshcomponent "/Game/Geometry/Meshes/1M_Cube.1M_Cube")
      (`SceneComponent.SetWorldScale3D` _itemmeshcomponent (0.25 0.25 1.0)))
    (:`AXE`
      (`StaticMeshComponent.SetStaticMesh` _itemmeshcomponent_2 "/Game/Geometry/Meshes/1M_Cube.1M_Cube")
      (`SceneComponent.SetWorldScale3D` _itemmeshcomponent_2 (0.5 0.5 1.0)))
    (:`SHIELD`
      (`StaticMeshComponent.SetStaticMesh` (`local.ItemMeshComponent`) "/Game/Meshes/Level/HexTile_mesh.HexTile_mesh"))))

(fn `UserConstructionScript`)