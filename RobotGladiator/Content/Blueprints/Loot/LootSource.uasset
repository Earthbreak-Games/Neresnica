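; Loot-drop source that spawns physics-launched pickups in a circle, scaled to player count, for Grunt and Boss enemies.
; ChooseItem rolls LootTable rarity and type, spawning health or data-table upgrades; bosses can also drop their own weapon, with random sword-part meshes.
; ClientUpdate events refresh loot widgets on clients and outline drops by rarity using custom-depth stencils and tinted line materials.
; Armor helpers exist, but ChooseItem never spawns armor.
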(event `DropLoot`
  (`self.ChooseItem`))

(event `ClientUpdateWeaponLoot`
  (params (Weapon :type "/Game/Blueprints/Loot/WeaponBP Object Reference"))
  (bind _rarity (`Weapon.Rarity` Weapon))
  (bind _lootline (`/Game/Blueprints/Loot/WeaponBP.LootLine` Weapon))
  (bind _rarity_2 (`Weapon.Rarity` Weapon))
  (bind _widget (`/Game/Blueprints/Loot/WeaponBP.Widget` Weapon))
  ;[1 1 1] Update Weapon Loot HUD on Client
  (`self.UpdateWeaponMesh` Weapon)
  (`/Engine/EditorBlueprintResources/StandardMacros.IsValid` _widget
    (:`Is Valid`
      (`SceneComponent.SetVisibility` _widget false false)
      (bind _asloot_hud_bp (cast `/Game/Blueprints/Loot/LootHUD_BP` (`WidgetComponent.GetWidget` _widget)))
      (`/Game/Blueprints/Loot/LootHUD_BP.SetBGColors` _asloot_hud_bp _rarity false)
      (`/Game/Blueprints/Loot/LootHUD_BP.SetHUDInfo` _asloot_hud_bp (`Weapon.WeaponName` Weapon) _rarity (`Weapon.WeaponType` Weapon) "HEAD" (`Weapon.BaseDamage` Weapon) false true)
      (`self.OutlineLootDrop` (`/Game/Blueprints/Loot/WeaponBP.Handle` Weapon) _lootline _rarity_2)
      (`self.OutlineLootDrop` (`/Game/Blueprints/Loot/WeaponBP.Hilt` Weapon) _lootline _rarity_2)
      (`self.OutlineLootDrop` (`/Game/Blueprints/Loot/WeaponBP.Blade` Weapon) _lootline _rarity_2))))

(event `ClientUpdateHealth`
  (params (HealthPack :type "Actor Object Reference"))
  ;[1 1 1] Update Health Loot HUD on Client
  (bind _ashealth_pickup (cast `/Game/Blueprints/Loot/HealthPickup` HealthPack))
  (bind _asloot_hud_bp (cast `/Game/Blueprints/Loot/LootHUD_BP` (`WidgetComponent.GetWidget` (`/Game/Blueprints/Loot/HealthPickup.Widget` _ashealth_pickup))))
  (`/Game/Blueprints/Loot/LootHUD_BP.SetBGColors` _asloot_hud_bp "COMMON" true)
  (`/Game/Blueprints/Loot/LootHUD_BP.SetHUDInfo` _asloot_hud_bp "None" "COMMON" "SWORD" "HEAD" (`KismetMathLibrary.FTrunc` (`/Game/Blueprints/Loot/HealthPickup.HealAmount` _ashealth_pickup)) true false)
  (`self.OutlineLootDrop` (`/Game/Blueprints/Loot/HealthPickup.Sphere` _ashealth_pickup) (`/Game/Blueprints/Loot/HealthPickup.LootLine` _ashealth_pickup) "COMMON" true))

(event `ClientUpdateArmorLoot`
  (params (Armor :type "/Game/Blueprints/Loot/ArmorBP Object Reference"))
  (bind _widget (`/Game/Blueprints/Loot/ArmorBP.Widget` Armor))
  (bind _rarity (`Armor.Rarity` Armor))
  (`SceneComponent.SetVisibility` _widget true false)
  (bind _asloot_hud_bp (cast `/Game/Blueprints/Loot/LootHUD_BP` (`WidgetComponent.GetWidget` _widget)))
  (`/Game/Blueprints/Loot/LootHUD_BP.SetBGColors` _asloot_hud_bp _rarity false)
  (`/Game/Blueprints/Loot/LootHUD_BP.SetHUDInfo` _asloot_hud_bp (`Armor.ArmorName` Armor) _rarity "SWORD" (`Armor.ArmorType` Armor) (`Armor.DefenseStat` Armor) false false)
  (`self.OutlineLootDrop` (`Armor.Mesh` Armor) null (`Armor.Rarity` Armor)))

(event `ClientUpdateUpgrade`
  (params (Upgrade :type "Actor Object Reference"))
  (bind _asupgrade_bp (cast `/Game/Blueprints/Loot/UpgradeBP` Upgrade))
  (bind _asupgrade_hud (cast `/Game/Blueprints/Loot/UpgradeHUD` (`WidgetComponent.GetWidget` (`/Game/Blueprints/Loot/UpgradeBP.Widget` _asupgrade_bp))))
  (bind _rarity (`Upgrade.Rarity` _asupgrade_bp))
  (`/Game/Blueprints/Loot/UpgradeHUD.SetBGColors` _asupgrade_hud _rarity)
  (`/Game/Blueprints/Loot/UpgradeHUD.SetHUDInfo` _asupgrade_hud (`Upgrade.UpgradeName` _asupgrade_bp))
  (`self.OutlineLootDrop` (`Upgrade.Mesh` _asupgrade_bp) (`/Game/Blueprints/Loot/UpgradeBP.LootLine` _asupgrade_bp) _rarity))

(fn `CalculateLootPosition`
  (params (Index :type Integer))
  (returns (Location :type "Vector Structure"))
  (bind _returnvalue (/ 360.0 (`KismetMathLibrary.Conv_IntToDouble` (`self.NumPlayers`))))
  (return (`KismetMathLibrary.GreaterGreater_VectorRotator` (`KismetMathLibrary.MakeVector` (`self.LootRaduis`)) (`KismetMathLibrary.MakeRotator` 0.0 0.0 (+ (* Index _returnvalue) (`KismetMathLibrary.MapRangeClamped` (`self.LootOffset`) 0.0 1.0 0.0 _returnvalue))))))

(fn `Choose UpgradeStat`
  (returns (UpgradeStat :type "EUpgradeStatType Enum"))
  (return (select `int` (`KismetMathLibrary.RandomIntegerInRange` 0 4) :`0` "SPEED" :`1` "JUMP" :`2` "ATTACKSPEED" :`3` "DAMAGE" :`4` "HEAL" :!type "EUpgradeStatType Enum")))

(fn `ChooseArmorType`
  (returns (ArmorType :type "EArmorTypes Enum"))
  (return (select `int` (`KismetMathLibrary.RandomIntegerInRange` 0 9) :`0` "HEAD" :`1` "HEAD" :`2` "HEAD" :`3` "HEAD" :`4` "HEAD" :`5` "CHEST" :`6` "CHEST" :`7` "CHEST" :`8` "CHEST" :`9` "CHEST" :!type "EArmorTypes Enum")))

(fn `ChooseItem`
  (locals (CompatibleItems :type "Array of Name") (SelectedRarity :type "ERarities Enum") (SelectedLootType :type "ELootTypes Enum") (LootLocation :type "Vector Structure") (BossWeaponData :type "/Game/Blueprints/Loot/WeaponDataStruct Structure") (ArmorDataList :type "Array of /Game/Blueprints/Loot/ArmorDataStruct Structure") (ArmorData :type "/Game/Blueprints/Loot/ArmorDataStruct Structure") (Rand :type Integer) (UpgradeDataList :type "Array of /Game/Blueprints/Loot/UpgradeDataStruct Structure") (UpgradeData :type "/Game/Blueprints/Loot/UpgradeDataStruct Structure"))
  (bind _compatibleitems (`local.CompatibleItems`))
  (bind (_name _rarity _weapontype _basedamage) (break `/Game/Blueprints/Loot/WeaponDataStruct` (`local.BossWeaponData`)))
  (bind (_name_2 _rarity_2 _upgradestat _affectedweapon _statincrease _stackincrease) (break `/Game/Blueprints/Loot/UpgradeDataStruct` (`local.UpgradeData`)))
  ;[1 1 1] Choose rarity
  (bind _returnvalue (`LootTable.ChooseRarity` (`self.LootTable`) 0.0))
  (set `local.SelectedRarity` _returnvalue)
  (switch `EEnemyTypes` (`self.EnemyType`)
    (:`GRUNT`
      (for _index (range (`self.NumPlayers`))
        ;[1 1 1] Calculate loot drop position
        (bind _location (`self.CalculateLootPosition` _index))
        (set `local.LootLocation` _location)
        ;[1 1 1] Choose item type based off of enemy
        (bind _returnvalue_2 (`LootTable.ChooseItemType` (`self.LootTable`) (`self.EnemyType`) 0.0))
        (bind _output_get (set `local.SelectedLootType` _returnvalue_2))
        (`KismetSystemLibrary.PrintString` (`|GetEnumeratorNameAsString` _output_get) true true (struct :`R` 0.1305 :`G` 0.063542 :`B` 1.0 :`A` 1.0))
        (switch `ELootTypes` _output_get :!label _label
          (:`HEALTH`
            ;[1 1 1] Drop Health
            (`KismetSystemLibrary.PrintString` "Health")
            (bind _returnvalue_3 (`|SpawnActorFromClass` "/Game/Blueprints/Loot/HealthPickup.HealthPickup_C" (`KismetMathLibrary.MakeTransform` (+ (`self.K2_GetActorLocation`) (`local.LootLocation`))) "Undefined" "OverrideRootScale" null null))
            ;[1 1 1] Setup loot HUD
            (bind _asloot_hud_bp (cast `/Game/Blueprints/Loot/LootHUD_BP` (`WidgetComponent.GetWidget` (`/Game/Blueprints/Loot/HealthPickup.Widget` _returnvalue_3))))
            (`/Game/Blueprints/Loot/LootHUD_BP.SetBGColors` _asloot_hud_bp "COMMON" true)
            (`/Game/Blueprints/Loot/LootHUD_BP.SetHUDInfo` _asloot_hud_bp "None" "COMMON" "SWORD" "HEAD" (`KismetMathLibrary.FTrunc` (`/Game/Blueprints/Loot/HealthPickup.HealAmount` _returnvalue_3)) true false)
            (`self.ClientUpdateHealth` _returnvalue_3)
            (bind _sphere (`/Game/Blueprints/Loot/HealthPickup.Sphere` _returnvalue_3))
            ;[1 1 1] Simulate physics
            (`PrimitiveComponent.SetSimulatePhysics` _sphere true)
            (`PrimitiveComponent.AddImpulse` _sphere (0.0 0.0 250.0) "None" true)
            (`PrimitiveComponent.AddRadialImpulse` _sphere (`self.K2_GetActorLocation`) 500.0 100.0 "RIF_Constant" true)
            (`self.SetLifeSpan` _returnvalue_3 (`self.LootLifeSpan`)))
          (:`UPGRADE`
            ;[1 1 1] Drop Upgrade
            (bind _upgradestat_2 (`self.Choose UpgradeStat`))
            (bind _outrownames (`DataTableFunctionLibrary.GetDataTableRowNames` "/Game/LootData/UpgradeDataTable.UpgradeDataTable"))
            (for _array_element _outrownames
              (bind _returnvalue_4 (`|GetDataTableRow` "/Game/LootData/UpgradeDataTable.UpgradeDataTable" _array_element)
                (:`then`
                  (bind (_name_3 _rarity_3 _upgradestat_3) (break `/Game/Blueprints/Loot/UpgradeDataStruct` _returnvalue_4))
                  (if (and (`|EnumEquality` _rarity_3 (`local.SelectedRarity`)) (`|EnumEquality` _upgradestat_3 _upgradestat_2))
                    (`KismetArrayLibrary.Array_Add` (`local.CompatibleItems`) _name_3)
                    (`KismetArrayLibrary.Array_Add` (`local.UpgradeDataList`) _returnvalue_4)))))
            (bind _output_get_2 (set `local.Rand` (`KismetMathLibrary.RandomIntegerInRange` 0 (`KismetArrayLibrary.Array_LastIndex` _compatibleitems))))
            (if (not (== (`|GetArrayItem` _compatibleitems _output_get_2) "None"))
              (set `local.UpgradeData` (`|GetArrayItem` (`local.UpgradeDataList`) _output_get_2))
              (bind _returnvalue_5 (`|SpawnActorFromClass` "/Game/Blueprints/Loot/UpgradeBP.UpgradeBP_C" (`KismetMathLibrary.MakeTransform` (+ (`self.K2_GetActorLocation`) (`local.LootLocation`))) "AlwaysSpawn" "OverrideRootScale" null "None" null))
              (`Upgrade.SetUpgradeStats` _returnvalue_5 _rarity_2 _upgradestat _affectedweapon _statincrease _stackincrease)
              (set `Upgrade.UpgradeName` _name_2 _returnvalue_5)
              (bind _asupgrade_hud (cast `/Game/Blueprints/Loot/UpgradeHUD` (`WidgetComponent.GetWidget` (`/Game/Blueprints/Loot/UpgradeBP.Widget` _returnvalue_5))))
              (`/Game/Blueprints/Loot/UpgradeHUD.SetBGColors` _asupgrade_hud _rarity_2)
              (`/Game/Blueprints/Loot/UpgradeHUD.SetHUDInfo` _asupgrade_hud _name_2)
              (`self.ClientUpdateUpgrade` _returnvalue_5)
              (bind _mesh (`Upgrade.Mesh` _returnvalue_5))
              ;[1 1 1] Simulate Physics
              (`PrimitiveComponent.SetSimulatePhysics` _mesh true)
              (`PrimitiveComponent.AddImpulse` _mesh (0.0 0.0 250.0) "None" true)
              (`PrimitiveComponent.AddRadialImpulse` _mesh (`self.K2_GetActorLocation`) 500.0 100.0 "RIF_Constant" true)
              (`self.SetLifeSpan` _returnvalue_5 (`self.LootLifeSpan`)))))))
    (:`BOSS`
      (`|ExecutionSequence`
        (:`then_0`
          (for _index_2 (range 1 (`self.NumPlayers`))
            ;[1 1 1] Calculate loot drop position
            (bind _location_2 (`self.CalculateLootPosition` _index_2))
            (set `local.LootLocation` _location_2)
            ;[1 1 1] Choose additional item type for boss to drop
            (bind _returnvalue_6 (`LootTable.ChooseItemType` (`self.LootTable`) "GRUNT" 0.0))
            (set `local.SelectedLootType` _returnvalue_6)
            (goto _label)))
        (:`then_1`
          ;[1 1 1] Calculate loot drop position
          (bind _location_3 (`self.CalculateLootPosition` 0))
          (set `local.LootLocation` _location_3)
          ;[1 1 1] Choose item type based off of enemy
          (bind _returnvalue_7 (`LootTable.ChooseItemType` (`self.LootTable`) (`self.EnemyType`) 0.0))
          (bind _output_get_3 (set `local.SelectedLootType` _returnvalue_7))
          (`KismetSystemLibrary.PrintString` (`|GetEnumeratorNameAsString` _output_get_3) true true (struct :`R` 0.1305 :`G` 0.063542 :`B` 1.0 :`A` 1.0))
          ;[1 1 1] Drop boss' current weapon
          (switch `ELootTypes` _output_get_3
            (:`WEAPON`
              (bind _outrownames_2 (`DataTableFunctionLibrary.GetDataTableRowNames` "/Game/LootData/WeaponDataTable.WeaponDataTable"))
              (for _array_element_2 _outrownames_2
                (bind _returnvalue_8 (`|GetDataTableRow` "/Game/LootData/WeaponDataTable.WeaponDataTable" _array_element_2)
                  (:`then`
                    (if (== (`.Name_2_B2B2B0EE4F506D39AB086C9C167C9782` (break `/Game/Blueprints/Loot/WeaponDataStruct` _returnvalue_8)) (`self.BossWeapon`))
                      (set `local.BossWeaponData` _returnvalue_8)
                      (break)))))
              (bind _returnvalue_9 (`|SpawnActorFromClass` "/Game/Blueprints/Loot/WeaponBP.WeaponBP_C" (`KismetMathLibrary.MakeTransform` (+ (`self.K2_GetActorLocation`) (`local.LootLocation`))) "AlwaysSpawn" "OverrideRootScale" null (`self.BossWeapon`) null))
              (`Weapon.SetWeaponStats` _returnvalue_9 _basedamage _rarity _weapontype)
              (`self.SelectWeaponMesh` _returnvalue_9 _rarity _weapontype)
              (bind _asloot_hud_bp_2 (cast `/Game/Blueprints/Loot/LootHUD_BP` (`WidgetComponent.GetWidget` (`/Game/Blueprints/Loot/WeaponBP.Widget` _returnvalue_9))))
              (`/Game/Blueprints/Loot/LootHUD_BP.SetBGColors` _asloot_hud_bp_2 _rarity false)
              (`/Game/Blueprints/Loot/LootHUD_BP.SetHUDInfo` _asloot_hud_bp_2 _name _rarity _weapontype "HEAD" _basedamage false true)
              (`self.ClientUpdateWeaponLoot` _returnvalue_9)
              (bind _handle (`/Game/Blueprints/Loot/WeaponBP.Handle` _returnvalue_9))
              (`PrimitiveComponent.SetSimulatePhysics` _handle true)
              (`PrimitiveComponent.AddImpulse` _handle (0.0 0.0 250.0) "None" true)
              (`PrimitiveComponent.AddRadialImpulse` _handle (`self.K2_GetActorLocation`) 500.0 100.0 "RIF_Constant" true)
              (`self.SetLifeSpan` _returnvalue_9 (`self.LootLifeSpan`)))))))))

(fn `ChooseWeaponType`
  (returns (WeaponType :type "EWeaponTypes Enum"))
  (return (select `int` (`KismetMathLibrary.RandomIntegerInRange` 0 9) :`0` "SWORD" :`1` "SWORD" :`2` "SWORD" :`3` "AXE" :`4` "AXE" :`5` "AXE" :`6` "AXE" :`7` "SWORD" :`8` "SWORD" :`9` "SWORD" :!type "EWeaponTypes Enum")))

(fn `GetRandomMesh`
  (params (MeshArray :type "Array of StaticMesh Object Reference"))
  (returns (SelectedMesh :type "StaticMesh Object Reference"))
  (return (`|GetArrayItem` MeshArray (`KismetMathLibrary.RandomIntegerInRange` 0 (- (`KismetArrayLibrary.Array_Length` MeshArray) 1)))))

(fn `OutlineLootDrop`
  (params (Mesh :type "StaticMeshComponent Object Reference") (LineMesh :type "StaticMeshComponent Object Reference") (Rarity :type "ERarities Enum" :default "COMMON") (IsHealth :type Boolean))
  (locals (LootMesh :type "StaticMeshComponent Object Reference") (Line :type "StaticMeshComponent Object Reference"))
  (set `local.LootMesh` Mesh)
  (set `local.Line` LineMesh)
  (if IsHealth
    ;[1 1 1] Outline Health Pack
    (`PrimitiveComponent.SetRenderCustomDepth` (`local.LootMesh`) true)
    (`PrimitiveComponent.SetCustomDepthStencilValue` (`local.LootMesh`) 0)
    (bind _returnvalue (`PrimitiveComponent.CreateDynamicMaterialInstance` (`local.Line`) 0 "/Game/Materials/Objects/LootLineMat.LootLineMat" "None"))
    (`MaterialInstanceDynamic.SetVectorParameterValue` _returnvalue "Color" (struct :`R` 1.0 :`B` 0.006201))
    (else
      (switch `ERarities` Rarity
        (:`COMMON`
          ;[1 1 1] Common item outline
          (`PrimitiveComponent.SetRenderCustomDepth` (`local.LootMesh`) true)
          (`PrimitiveComponent.SetCustomDepthStencilValue` (`local.LootMesh`) 1)
          (bind _returnvalue_2 (`PrimitiveComponent.CreateDynamicMaterialInstance` (`local.Line`) 0 "/Game/Materials/Objects/LootLineMat.LootLineMat" "None"))
          (`MaterialInstanceDynamic.SetVectorParameterValue` _returnvalue_2 "Color" (struct :`G` 1.0 :`B` 0.129594)))
        (:`RARE`
          ;[1 1 1] Rare item outline
          (`PrimitiveComponent.SetRenderCustomDepth` (`local.LootMesh`) true)
          (`PrimitiveComponent.SetCustomDepthStencilValue` (`local.LootMesh`) 2)
          (bind _returnvalue_3 (`PrimitiveComponent.CreateDynamicMaterialInstance` (`local.Line`) 0 "/Game/Materials/Objects/LootLineMat.LootLineMat" "None"))
          (`MaterialInstanceDynamic.SetVectorParameterValue` _returnvalue_3 "Color" (struct :`R` 0.005822 :`G` 0.416935 :`B` 1.0)))
        (:`LEGENDARY`
          ;[1 1 1] Legendary item outline
          (`PrimitiveComponent.SetRenderCustomDepth` (`local.LootMesh`) true)
          (`PrimitiveComponent.SetCustomDepthStencilValue` (`local.LootMesh`) 3)
          (bind _returnvalue_4 (`PrimitiveComponent.CreateDynamicMaterialInstance` (`local.Line`) 0 "/Game/Materials/Objects/LootLineMat.LootLineMat" "None"))
          (`MaterialInstanceDynamic.SetVectorParameterValue` _returnvalue_4 "Color" (struct :`R` 0.885442 :`B` 1.0)))
        (:`EPIC`
          ;[1 1 1] Epic item outline
          (`PrimitiveComponent.SetRenderCustomDepth` (`local.LootMesh`) true)
          (`PrimitiveComponent.SetCustomDepthStencilValue` (`local.LootMesh`) 4))))))

(fn `SelectArmorMesh`
  (params (MeshComponent :type "StaticMeshComponent Object Reference") (Rarity :type "ERarities Enum" :default "COMMON") (ArmorType :type "EArmorTypes Enum" :default "HEAD"))
  (locals (ItemMeshComponent :type "StaticMeshComponent Object Reference"))
  (bind _itemmeshcomponent (`local.ItemMeshComponent`))
  (bind _itemmeshcomponent_2 (`local.ItemMeshComponent`))
  (bind _itemmeshcomponent_3 (`local.ItemMeshComponent`))
  (set `local.ItemMeshComponent` MeshComponent)
  (switch `EArmorTypes` ArmorType
    (:`HEAD`
      (`StaticMeshComponent.SetStaticMesh` _itemmeshcomponent_2 "/Game/DefaultContent/Geometry/Meshes/1M_Cube.1M_Cube")
      (`SceneComponent.SetWorldScale3D` _itemmeshcomponent_2 (0.5 0.5 0.5)))
    (:`CHEST`
      (`StaticMeshComponent.SetStaticMesh` (`local.ItemMeshComponent`) "/Game/DefaultContent/Geometry/Meshes/1M_Cube.1M_Cube"))
    (:`ARMS`
      (`StaticMeshComponent.SetStaticMesh` _itemmeshcomponent_3 "/Game/DefaultContent/Geometry/Meshes/1M_Cube.1M_Cube")
      (`SceneComponent.SetWorldScale3D` _itemmeshcomponent_3 (0.5 0.5 0.25)))
    (:`LEGS`
      (`StaticMeshComponent.SetStaticMesh` _itemmeshcomponent "/Game/DefaultContent/Geometry/Meshes/1M_Cube.1M_Cube")
      (`SceneComponent.SetWorldScale3D` _itemmeshcomponent (0.5 0.5 1.0)))))

(fn `SelectWeaponMesh`
  (params (Weapon :type "/Game/Blueprints/Loot/WeaponBP Object Reference") (Rarity :type "ERarities Enum" :default "COMMON") (WeaponType :type "EWeaponTypes Enum" :default "SWORD"))
  (locals (ItemMeshComponent :type "StaticMeshComponent Object Reference"))
  (bind _hilt (`/Game/Blueprints/Loot/WeaponBP.Hilt` Weapon))
  (bind _handle (`/Game/Blueprints/Loot/WeaponBP.Handle` Weapon))
  (bind _blade (`/Game/Blueprints/Loot/WeaponBP.Blade` Weapon))
  (switch `EWeaponTypes` WeaponType
    (:`SWORD`
      (bind _selectedmesh (`self.GetRandomMesh` (`self.SwordHandles`)))
      (bind _output_get (set `/Game/Blueprints/Loot/WeaponBP.HandleMesh` _selectedmesh Weapon))
      (`StaticMeshComponent.SetStaticMesh` _handle _output_get)
      (`SceneComponent.SetWorldScale3D` _handle (0.4 0.4 0.4))
      (bind _selectedmesh_2 (`self.GetRandomMesh` (`self.SwordHilts`)))
      (bind _output_get_2 (set `/Game/Blueprints/Loot/WeaponBP.HiltMesh` _selectedmesh_2 Weapon))
      (`StaticMeshComponent.SetStaticMesh` _hilt _output_get_2)
      (`SceneComponent.SetWorldScale3D` _hilt (0.4 0.4 0.4))
      (bind _selectedmesh_3 (`self.GetRandomMesh` (`self.SwordBlades`)))
      (bind _output_get_3 (set `/Game/Blueprints/Loot/WeaponBP.BladeMesh` _selectedmesh_3 Weapon))
      (`StaticMeshComponent.SetStaticMesh` _blade _output_get_3)
      (`SceneComponent.SetWorldScale3D` _blade (0.4 0.4 0.4)))))

(fn `UpdateWeaponMesh`
  (params (Weapon :type "/Game/Blueprints/Loot/WeaponBP Object Reference"))
  (bind _handle (`/Game/Blueprints/Loot/WeaponBP.Handle` Weapon))
  (bind _hilt (`/Game/Blueprints/Loot/WeaponBP.Hilt` Weapon))
  (bind _blade (`/Game/Blueprints/Loot/WeaponBP.Blade` Weapon))
  (`StaticMeshComponent.SetStaticMesh` _handle (`/Game/Blueprints/Loot/WeaponBP.HandleMesh` Weapon))
  (`SceneComponent.SetWorldScale3D` _handle (0.4 0.4 0.4))
  (`StaticMeshComponent.SetStaticMesh` _hilt (`/Game/Blueprints/Loot/WeaponBP.HiltMesh` Weapon))
  (`SceneComponent.SetWorldScale3D` _hilt (0.4 0.4 0.4))
  (`StaticMeshComponent.SetStaticMesh` _blade (`/Game/Blueprints/Loot/WeaponBP.BladeMesh` Weapon))
  (`SceneComponent.SetWorldScale3D` _blade (0.4 0.4 0.4)))

(fn `UserConstructionScript`)