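; LobbySpawnPoints is a level actor that places players and assigns their cameras in the lobby.
; FindOpenSpawnPoint claims the first unoccupied entry in SpawnPoints and returns it offset by the actor's location.
; SetSpawnPositions moves each controller's pawn to the spawn point matching its index, and SetLobbyCameras gives each ThirdPersonCharacter its matching LobbyCamera.
; BeginPlay caches the first BPArenaGrid, which no graph here uses.
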(event `self.ReceiveBeginPlay`
  (bind _outactors (`GameplayStatics.GetAllActorsOfClass` "/Game/Blueprints/Level/BPArenaGrid.BPArenaGrid_C"))
  (set `self.Grid` (`|GetArrayItem` _outactors)))

(event `self.ReceiveTick`
  (params (DeltaSeconds :type "Float (single-precision)")))

(fn `FindOpenSpawnPoint`
  (returns (SpawnLoc :type "Vector Structure"))
  (bind _occupiedpoints (`self.OccupiedPoints`))
  (for (_array_element _array_index) (`self.SpawnPoints`)
    (if (not (`|GetArrayItem` _occupiedpoints _array_index))
      (`KismetArrayLibrary.Array_Set` _occupiedpoints _array_index true)
      (return (+ _array_element (`self.K2_GetActorLocation`))))))

(fn `SetLobbyCameras`
  (params (PlayerControllers :type "Array of /Game/Character/Blueprints/CharacterController Object Reference"))
  (for (_array_element _array_index) PlayerControllers
    (bind _asthird_person_character (cast `/Game/Character/Blueprints/ThirdPersonCharacter` (`PlayerState.PawnPrivate` (`Controller.PlayerState` _array_element))))
    (set `/Game/Character/Blueprints/ThirdPersonCharacter.LobbyCamera` (`|GetArrayItem` (`self.LobbyCameras`) _array_index) _asthird_person_character)))

(fn `SetSpawnPositions`
  (params (PlayerControllers :type "Array of PlayerController Object Reference"))
  (for (_array_element _array_index) PlayerControllers
    (bind _pawnprivate (`PlayerState.PawnPrivate` (`Controller.PlayerState` _array_element)))
    (`/Engine/EditorBlueprintResources/StandardMacros.IsValid` _pawnprivate
      (:`Is Valid`
        (`self.K2_SetActorLocation` _pawnprivate (+ (`|GetArrayItem` (`self.SpawnPoints`) _array_index) (`self.K2_GetActorLocation`)) false false)))))

(fn `UserConstructionScript`)