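; Toxic Topper is a hex-tile topper that seeds neighboring tiles with Jump Toppers and reacts to player overlap.
; On BeginPlay it traces down to its hex, then traces toward six fixed offsets to find neighbors.
; It takes the first hits up to SideSpawns, without shuffling, and spawns Jump Toppers high above them, matching its own hex's rotation.
; Overlapping a ThirdPersonCharacter calls DealDamage with zero damage.
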(event `self.ReceiveBeginPlay`
  (bind _height_offset (`self.Height_offset`))
  (bind _returnvalue (`self.K2_GetActorLocation` self))
  ;[1 1 1] Spawn Neighboring Nodes
  (bind _outhit (`KismetSystemLibrary.LineTraceSingle` :`Start` _returnvalue :`End` (+ _returnvalue (0.0 0.0 -100.0)) :`TraceChannel` "TraceTypeQuery1" :`DrawDebugType` "Persistent"))
  (set `self.Found_Hex` (`|MakeArray`))
  (bind (_bblockinghit _binitialoverlap _time _distance _location _impactpoint _normal _impactnormal _physmat _hitactor) (`GameplayStatics.BreakHitResult` _outhit))
  (bind _returnvalue_2 (`SceneComponent.K2_GetComponentLocation` (`Actor.RootComponent` _hitactor)))
  (for _array_element (`|MakeArray` (+ _returnvalue_2 (-210.0 350.0 0.0)) (+ _returnvalue_2 (210.0 350.0 0.0)) (+ _returnvalue_2 (210.0 -350.0 0.0)) (+ _returnvalue_2 (-400.0 0.0 0.0)) (+ _returnvalue_2 (400.0 0.0 0.0)) (+ _returnvalue_2 (-210.0 -350.0 0.0)))
    (bind (_outhit_2 _returnvalue_3) (`KismetSystemLibrary.LineTraceSingle` (+ _returnvalue_2 _height_offset) (+ _array_element _height_offset) "TraceTypeQuery1" false (`|MakeArray` _hitactor) "Persistent"))
    (if _returnvalue_3
      (`KismetArrayLibrary.Array_Add` (`self.Found_Hex`) (`.HitActor` (`GameplayStatics.BreakHitResult` _outhit_2)))))
  (set `self.chosen_hex` (`|MakeArray`))
  (for _array_element_2 (`self.Found_Hex`)
    (if (< (`KismetArrayLibrary.Array_Length` (`self.chosen_hex`)) (`self.Side Spawns`))
      (`KismetArrayLibrary.Array_Add` (`self.chosen_hex`) _array_element_2)))
  (for _array_element_3 (`self.chosen_hex`)
    (bind _returnvalue_4 (`|SpawnActorFromClass` "/Game/Blueprints/Level/Jump_Topper.Jump_Topper_C" (`KismetMathLibrary.Conv_VectorToTransform` (+ (`SceneComponent.K2_GetComponentLocation` (`Actor.RootComponent` _array_element_3)) (0.0 0.0 1500.0))) "Undefined" "OverrideRootScale" null null))
    (`self.K2_SetActorRotation` _returnvalue_4 (`self.K2_GetActorRotation` _hitactor) false)))

(event `self.ReceiveActorBeginOverlap`
  (params (OtherActor :type "Actor Object Reference"))
  (bind _asthird_person_character (cast `/Game/Characters/Player/Blueprints/ThirdPersonCharacter` OtherActor))
  (`BaseUnit.DealDamage` _asthird_person_character null 0.0))

(fn `UserConstructionScript`)