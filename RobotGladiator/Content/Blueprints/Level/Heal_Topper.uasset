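; Heal Topper is a level actor that heals a ThirdPersonCharacter that overlaps it.
; On begin overlap, it computes a heal amount as the Hp percentage of the character's max health.
; A while loop with a latent Delay in its body calls Heal while health is below max, with debug prints.
; No end-overlap handling exists, so leaving the actor does not cancel healing.
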(event `self.ReceiveActorBeginOverlap`
  (params (OtherActor :type "Actor Object Reference"))
  (bind _asthird_person_character (cast `/Game/Characters/Player/Blueprints/ThirdPersonCharacter` OtherActor))
  (bind _mmaxhealth (`BaseUnit.mMaxHealth` _asthird_person_character))
  (`KismetSystemLibrary.PrintString` (`KismetStringLibrary.Conv_DoubleToString` _mmaxhealth))
  (set `self.Heal ammount` (* (* (`self.Hp %`) 0.01) _mmaxhealth))
  (bind _returnvalue (< (`BaseUnit.mHealth` _asthird_person_character) _mmaxhealth))
  (`KismetSystemLibrary.PrintString` (`KismetStringLibrary.Conv_BoolToString` _returnvalue))
  (while _returnvalue
    (`KismetSystemLibrary.Delay` (`self.Delay`))
    (`BaseUnit.Heal` _asthird_person_character (`self.Heal ammount`))
    (`KismetSystemLibrary.PrintString` "Healing")))

(fn `UserConstructionScript`)