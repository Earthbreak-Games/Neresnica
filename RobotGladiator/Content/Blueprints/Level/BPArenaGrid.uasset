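; Arena floor grid that spawns cell tiles and animates their heights for lobby and round transitions.
; Custom events generate, randomize, save, load and erase height layouts by index.
; Tick runs flag-driven steps that VInterp tiles toward saved heights, move the center tile and lobby ring separately, and reset materials after a round.
; Raising the center tile back up triggers EndRound.
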(event `self.ReceiveBeginPlay`
  ;[1 1 1] Set CenterTile
  (set `self.CenterTile` (`|GetArrayItem` (`self.FloorPieces`)))
  (bind _result (`/Engine/EditorBlueprintResources/StandardMacros.DecrementInt` (`KismetArrayLibrary.Array_Length` (`self.SavedStates`)))
    (:`  `
      (set `self.NumSavedStates` _result))))

(event `GenerateArenaFloor`
  ;[1 1 1] Generate the arena's floor
  (`self.ClearFloor`)
  (`self.SpawnFloor` (`self.K2_GetActorLocation`) (`self.Radius`) (`self.Padding`))
  (`self.SetupLobbyOrientation` 7)
  (bind _asarena_floor_cell (cast `/Game/Blueprints/Level/ArenaFloorCell` (`|GetArrayItem` (`self.FloorPieces`))))
  (`PrimitiveComponent.SetMaterial` (`/Game/Blueprints/Level/ArenaFloorCell.Pillar` _asarena_floor_cell) 0 "/Game/Materials/Prototype/SafeZoneTest.SafeZoneTest"))

(event `self.ReceiveTick`
  (params (DeltaSeconds :type "Float (single-precision)"))
  (bind _maxheight (`self.MaxHeight`))
  (bind _centertile (`self.CenterTile`))
  (bind _centertile_2 (`self.CenterTile`))
  (bind (_returnvalue_x _returnvalue_y _returnvalue_z) (`KismetMathLibrary.BreakVector` (`self.K2_GetActorLocation` _centertile_2)))
  (bind (_returnvalue_x_2 _returnvalue_y_2 _returnvalue_z_2) (`KismetMathLibrary.BreakVector` (`self.K2_GetActorLocation` _centertile)))
  (`|ExecutionSequence`
    (:`then_0`
      ;[1 1 1] Reset all tile's materials to the default material
      (if (`self.RoundEnded`)
        (for _array_element (`self.FloorPieces`)
          (if (not (== _array_element (`self.CenterTile`)))
            (bind _asarena_floor_cell (cast `/Game/Blueprints/Level/ArenaFloorCell` _array_element))
            (`/Engine/EditorBlueprintResources/StandardMacros.IsValid` _asarena_floor_cell
              (:`Is Valid`
                (`PrimitiveComponent.SetMaterial` (`/Game/Blueprints/Level/ArenaFloorCell.Pillar` _asarena_floor_cell) 0 "/Game/Materials/Prototype/TestDefault.TestDefault")))))
        (set `self.RoundEnded` false)))
    (:`then_1`
      ;[1 1 1] Move tiles to the correct height
      (if (`self.UpdateTiles`)
        (if (`self.ArenaIncrementFlag`)
          (`self.LoadSaveState` (`self.CurSavedState`) (`self.NoiseScale`))
          (set `self.ArenaIncrementFlag` false))
        ;;[1 1 1] Move arena tiles
        (for (_array_element_2 _array_index) (`self.FloorPieces`)
          (if (not (== _array_element_2 (`self.CenterTile`)))
            (`self.MoveTile` _array_element_2 (`|GetArrayItem` (`self.FloorHeights`) _array_index) 1.0)))
        (else
          (set `self.ArenaIncrementFlag` true))))
    (:`then_2`
      ;[1 1 1] Lower the center tile to the min height
      (if (and (`self.UpdateCenterTile`) (not (`self.ResetCenter`)))
        (`self.MoveTile` _centertile_2 (`self.MinHeight`) 1.0)
        (if (<= _returnvalue_z 1.0)
          (`self.K2_SetActorLocation` _centertile_2 (`KismetMathLibrary.MakeVector` _returnvalue_x _returnvalue_y (`self.MinHeight`)) false false)
          (set `self.UpdateCenterTile` false))))
    (:`then_3`
      ;[1 1 1] Reset center tile to it's original position
      (if (`self.ResetCenter`)
        (`self.MoveTile` _centertile (`self.MaxHeight`) 1.0)
        (if (>= _returnvalue_z_2 1495.0)
          (set `self.ResetCenter` false)
          ;[1 1 1] Start round ending sequence
          (`self.EndRound`)
          (set `self.UpdateTiles` false)
          (set `self.UpdateCenterTile` false)
          (set `self.RoundEnded` true))))
    (:`then_4`
      ;[1 1 1] Move first ring of tiles
      (if (`self.ExitLobby`)
        (for _index (range (`self.NumLobbyTiles`))
          (bind _output (`|GetArrayItem` (`self.FloorPieces`) _index))
          (`self.MoveTile` _output _maxheight 0.25)
          (bind (_returnvalue_x_3 _returnvalue_y_3 _returnvalue_z_3) (`KismetMathLibrary.BreakVector` (`self.K2_GetActorLocation` _output)))
          (if (>= _returnvalue_z_3 (- _maxheight 5.0))
            (`self.K2_SetActorLocation` _output (`KismetMathLibrary.MakeVector` _returnvalue_x_3 _returnvalue_y_3 (`self.MaxHeight`)) false false)))))
    (:`then_5`
      ;[1 1 1] Reset center ring of tiles
      (if (`self.ResetCenterRing`)
        (for _index_2 (range 1 (`self.NumLobbyTiles`))
          (`self.MoveTile` (`|GetArrayItem` (`self.FloorPieces`) _index_2) (`self.MinHeight`) 1.0))))))

(event `ClearArenaFloor`
  ;[1 1 1] Clear the arena's floor
  (`self.ClearFloor`))

(event `SaveCurrentLevel`
  ;[1 1 1] Save the arena to the current index
  (`self.SaveState` (`self.WorkingIndex`) false))

(event `RandomizeHeights`
  ;[1 1 1] Load a fresh randomly generated arena
  (`self.GenerateArena` (`self.TopperChance`) (`self.NoiseScale`))
  (bind _returnvalue (`self.SaveState` -1))
  (`self.ClearFloor`)
  (bind _output_get (set `self.WorkingIndex` _returnvalue))
  (`self.EditorLoadSaveState` _output_get (`self.K2_GetActorLocation`) (`self.Radius`) (`self.Padding`)))

(event `ClearSavedState`
  ;[1 1 1] Erase the save state at the selected index
  (`self.EraseHeightState` (`self.WorkingIndex`))
  (set `self.WorkingIndex` (- (`KismetArrayLibrary.Array_Length` (`self.SavedStates`)) 1)))

(event `LoadSavedState`
  ;[1 1 1] Load the state at the given index
  (`self.ClearFloor`)
  (`self.EditorLoadSaveState` (`self.WorkingIndex`) (`self.K2_GetActorLocation`) (`self.Radius`) (`self.Padding`)))

(fn `MoveTile`
  (params (Tile :type "Actor Object Reference") (EndHeight :type "Float (double-precision)") (Speed :type "Float (double-precision)"))
  (bind _asarena_floor_cell (cast `/Game/Blueprints/Level/ArenaFloorCell` Tile))
  (`/Engine/EditorBlueprintResources/StandardMacros.IsValid` _asarena_floor_cell
    (:`Is Valid`
      (bind _returnvalue (`self.K2_GetActorLocation` _asarena_floor_cell))
      (`self.K2_SetActorLocation` _asarena_floor_cell (`KismetMathLibrary.VInterpTo` _returnvalue (`KismetMathLibrary.MakeVector` (.x _returnvalue) (.y _returnvalue) EndHeight) (`GameplayStatics.GetWorldDeltaSeconds`) Speed) false false))))

(fn `UserConstructionScript`)