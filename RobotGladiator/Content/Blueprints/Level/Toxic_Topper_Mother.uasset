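; Toxic Topper Mother is a level hazard that deals periodic damage to ThirdPersonCharacters standing inside its collision area.
; Overlap adds the character to a damage list, opens a gate and starts a Delay loop that damages every listed character through HostNotifyDealDamage.
; Any listed character leaving is removed and closes the gate, halting the repeat even if others remain inside.
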(event `self.ReceiveActorBeginOverlap`
  (params (OtherActor :type "Actor Object Reference")))

(event `self.Collision Area.OnComponentBeginOverlap`
  (params (OverlappedComponent :type "PrimitiveComponent Object Reference") (OtherActor :type "Actor Object Reference") (OtherComp :type "PrimitiveComponent Object Reference") (OtherBodyIndex :type Integer) (bFromSweep :type Boolean) (SweepResult :type "HitResult Structure (by ref)"))
  (bind _asthird_person_character (cast `/Game/Characters/Player/Blueprints/ThirdPersonCharacter` OtherActor))
  (`KismetArrayLibrary.Array_Add` (`self.PlayersToDamage`) _asthird_person_character)
  (`|ExecutionSequence`
    (:`then_0`
      (goto _label_2 :!via `Open`))
    (:`then_1`
      (`KismetSystemLibrary.Delay` (`self.Delay`) :!label _label)
      (`self.DamagePlayer`)
      (`/Engine/EditorBlueprintResources/StandardMacros.Gate` true :!label _label_2
        (:`Exit`
          (goto _label))))))

(event `self.Collision Area.OnComponentEndOverlap`
  (params (OverlappedComponent :type "PrimitiveComponent Object Reference") (OtherActor :type "Actor Object Reference") (OtherComp :type "PrimitiveComponent Object Reference") (OtherBodyIndex :type Integer))
  (bind _playerstodamage (`self.PlayersToDamage`))
  (bind _asthird_person_character (cast `/Game/Characters/Player/Blueprints/ThirdPersonCharacter` OtherActor))
  (bind _returnvalue (`KismetArrayLibrary.Array_Find` _playerstodamage _asthird_person_character))
  (if (!= _returnvalue -1)
    (`KismetArrayLibrary.Array_Remove` _playerstodamage _returnvalue)
    (goto _label_2 :!via `Close`)))

(event `DamagePlayer`
  (for _array_element (`self.PlayersToDamage`)
    (`/Game/Characters/Player/Blueprints/ThirdPersonCharacter.HostNotifyDealDamage` _array_element _array_element (`self.Damage`) false false)))

(fn `UserConstructionScript`)