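; Parent Blueprint for a level topper spawner, which places an actor of its Topper class in relation to the actor beneath it.
; On BeginPlay it traces downward with persistent debug drawing, spawns the Topper high above the hit actor's root and copies that root's rotation.
; A disconnected, never-run branch would ease this actor down to the Arena's minimum height.
; Tick, the construction script and the Topper OnRep are empty.
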(event `self.ReceiveBeginPlay`
  (bind _returnvalue (`self.K2_GetActorLocation` self))
  (bind _outhit (`KismetSystemLibrary.LineTraceSingle` :`Start` _returnvalue :`End` (+ _returnvalue (0.0 0.0 -400.0)) :`TraceChannel` "TraceTypeQuery1" :`DrawDebugType` "Persistent"))
  (bind _rootcomponent (`Actor.RootComponent` (`.HitActor` (`GameplayStatics.BreakHitResult` _outhit))))
  (bind _returnvalue_2 (`|SpawnActorFromClass` (`self.Topper`) (`KismetMathLibrary.Conv_VectorToTransform` (+ (`SceneComponent.K2_GetComponentLocation` _rootcomponent) (0.0 0.0 1500.0))) "AlwaysSpawn" "OverrideRootScale" null null))
  (`self.K2_SetActorRotation` _returnvalue_2 (`SceneComponent.K2_GetComponentRotation` _rootcomponent) false))

(event `self.ReceiveTick`
  (params (DeltaSeconds :type "Float (single-precision)")))

(fn `OnRep_Topper`)

(fn `UserConstructionScript`)