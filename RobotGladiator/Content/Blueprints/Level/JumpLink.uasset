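; JumpLink is a smart nav link that makes TestNavCaracter agents jump to the link's destination.
; On reaching it, CalculateVelocity solves a ballistic launch velocity from JumpDuration and hardcoded gravity, then the agent stops moving, launches and is flagged as jumping.
; A separate Jump event launches a passed character the same way, but computes velocity from the link's location to world origin.
; Debug prints show the velocity and overlaps.
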(event `self.ReceiveSmartLinkReached`
  (params (Agent :type "Actor Object Reference") (Destination :type "Vector Structure (by ref)"))
  (bind _vel (`self.CalculateVelocity` Destination (`self.K2_GetActorLocation` Agent) (`self.Jump Duration`)))
  (`KismetSystemLibrary.PrintString` (`KismetStringLibrary.Conv_VectorToString` _vel))
  (bind _astest_nav_caracter (cast `/Game/Characters/TestNavCaracter` Agent))
  (`NavMovementComponent.StopActiveMovement` (`Character.CharacterMovement` _astest_nav_caracter))
  (`Character.LaunchCharacter` _astest_nav_caracter _vel true true)
  (set `/Game/Characters/TestNavCaracter.IsJumping` true _astest_nav_caracter))

(event `self.ReceiveActorBeginOverlap`
  (params (OtherActor :type "Actor Object Reference"))
  (`KismetSystemLibrary.PrintString` "Hello"))

(event `Jump`
  (params (NewParam :type "Actor Object Reference"))
  (bind _vel (`self.CalculateVelocity` (0.0 0.0 0.0) (`self.K2_GetActorLocation`) (`self.Jump Duration`)))
  (`KismetSystemLibrary.PrintString` (`KismetStringLibrary.Conv_VectorToString` _vel))
  (bind _astest_nav_caracter (cast `/Game/Characters/TestNavCaracter` NewParam))
  (`NavMovementComponent.StopActiveMovement` (`Character.CharacterMovement` _astest_nav_caracter))
  (`Character.LaunchCharacter` _astest_nav_caracter _vel true true)
  (set `/Game/Characters/TestNavCaracter.IsJumping` true _astest_nav_caracter))

(fn `CalculateVelocity`
  (params (Dest :type "Vector Structure") (Start :type "Vector Structure") (Dur :type "Float (double-precision)"))
  (returns (Vel :type "Vector Structure"))
  (locals (indur :type "Float (double-precision)"))
  (bind _output_get (set `local.indur` Dur))
  (return (`KismetMathLibrary.MakeVector` (/ (- (.x Dest) (.x Start)) _output_get) (/ (- (.y Dest) (.y Start)) _output_get) (/ (- (.z Dest) (+ (.z Start) (* (`KismetMathLibrary.Square` (`local.indur`)) -0.5 982.0))) (`local.indur`)))))

(fn `UserConstructionScript`)