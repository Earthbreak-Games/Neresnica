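; Temporary arena tile topper that lowers itself back to the arena grid's minimum height when flagged for reset.
; On BeginPlay it caches its attach parent as the BPArenaGrid.
; While Reset is set, Tick eases Z toward the grid's MinHeight with VInterpTo.
; Within one unit of the target, it sets a final location from only X and Y, leaving Z unwired, and clears Reset.
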(event `self.ReceiveBeginPlay`
  (bind _asbparena_grid (cast `/Game/Blueprints/Level/BPArenaGrid` (`self.GetAttachParentActor`)))
  (set `self.Arena` _asbparena_grid))

(event `self.ReceiveTick`
  (params (DeltaSeconds :type "Float (single-precision)"))
  (bind _returnvalue (`self.K2_GetActorLocation`))
  (bind (_returnvalue_x _returnvalue_y) (`KismetMathLibrary.BreakVector` (`self.K2_GetActorLocation`)))
  (bind (_returnvalue_x_2 _returnvalue_y_2 _returnvalue_z) (`KismetMathLibrary.BreakVector` (`self.K2_GetActorLocation`)))
  (bind _returnvalue_2 (`KismetMathLibrary.MakeVector` (.x _returnvalue) (.y _returnvalue) (`ArenaGrid.MinHeight` (`self.Arena`))))
  ;[1 1 1] Reset this tile's height to the min height
  (if (`self.Reset`)
    (`self.K2_SetActorLocation` (`KismetMathLibrary.VInterpTo` _returnvalue _returnvalue_2 (`GameplayStatics.GetWorldDeltaSeconds`) 1.0))
    (if (<= (`KismetMathLibrary.Abs` (- _returnvalue_z (.z _returnvalue_2))) 1.0)
      (`self.K2_SetActorLocation` (`KismetMathLibrary.MakeVector` _returnvalue_x _returnvalue_y))
      (set `self.Reset` false))))

(fn `UserConstructionScript`)